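; BP_Enemy_Locn is a location marker for the robot enemy Blueprint, shown in the scene as either a Start or an End node.
; Its construction script calls a Construction function, kept separate so other Blueprints can also trigger it.
; That function sets the text label and creates a dynamic billboard material, choosing the start or end texture from the Start flag.
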(fn ConstructionScript
  ;[0 1 0] Construction has been placed into a function to allow it to be called from outside the BP
  (CallFunction|Construction))

(fn Construction
  ;[1 1 0] Setup the appropriate Material Billboard texture used in Scene dependent on whether this is a Start or an End Node. Used by Enemy Robot BP
  (Rendering|Components|TextRender|SetText (Variables|Default|GetTextRender) (Variables|Default|GetText))
  (bind _returnvalue (Rendering|Material|CreateDynamicMaterialInstance (Variables|Default|GetMaterialBillboard) 0 "/Game/PlatformTools/Characters/RobotEnemy/Materials/MI_EnemyLoc_Billboard.MI_EnemyLoc_Billboard" "None" :!class /Script/Engine.PrimitiveComponent))
  (if (Variables|Default|GetStart?)
    (Rendering|Material|SetTextureParameterValue _returnvalue "Texture" (Variables|Default|GetStartTexture))
    (else
      (Rendering|Material|SetTextureParameterValue _returnvalue "Texture" (Variables|Default|GetEndTexture)))))