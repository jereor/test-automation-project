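; Robot enemy for a platformer that patrols along X between two endpoints, which the construction script line-traces and marks with child actors.
; A looping timeline drives both movement and the mask's flipbook material.
; Player contact damages both sides and reverses direction, while projectile hits turn it toward the player, with self-damage scaled by player class and level.
; Hits flash a shield material, and death plays particles, reports a goal and destroys the actor.
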(event OnComponentBeginOverlap(CapsuleCollision)
  (params (OverlappedComponent :type Primitive%20Component%20Object%20Reference) (OtherActor :type Actor%20Object%20Reference) (OtherComp :type Primitive%20Component%20Object%20Reference) (OtherBodyIndex :type Integer) (bFromSweep :type Boolean) (SweepResult :type Hit%20Result%20Structure%20%28by%20ref%29))
  (bind _returnvalue (Game|GetPlayerCharacter 0))
  (bind _bpplatformercomponent (Variables|Default|GetBPPlatformerComponent))
  ;[0 1 0] Player or Projectile Collision with Enemy
  (Utilities|FlowControl|Sequence
    (:then_0
      (Utilities|IsValid _returnvalue
        (:Is%20Valid
          (if (== OtherActor _returnvalue)
            (Variables|Default|SetPlayerCollision true)
            (Utilities|FlowControl|DoOnce false
              (:Completed
                (Utilities|IsValid _bpplatformercomponent
                  (:Is%20Valid
                    (Default|CallApplyDamageEvent _bpplatformercomponent (Variables|Default|GetPlayerDamage))
                    (if (Variables|Default|GetPlayerCollision) :!label _label
                      (Variables|Default|SetForward (not (Variables|Default|GetForward)))
                      (else
                        (CallFunction|FacePlayer)))
                    (Rendering|Material|SetMaterial (Variables|Character|GetMesh) 0 (Variables|Default|GetDMI_Damage))
                    (Game|Damage|ApplyDamage self (* (Variables|Default|GetSelfDamage) (Variables|Default|GetDamageMultiplier)) 0 0)
                    (Rendering|Material|SetVectorParameterValue (Variables|Default|GetDMI_RobotMask) "Color" (Variables|Appearance|GetFlipbookTextureColor_Angry) :!class /Script/Engine.MaterialInstanceDynamic)
                    (CallFunction|ResetDamage)
                    (Utilities|FlowControl|Delay 0.2)
                    (Utilities|IsValid (Variables|Character|GetMesh)
                      (:Is%20Valid
                        (Rendering|Material|SetMaterial (Variables|Character|GetMesh) 0 (Variables|Default|GetMI_Slot0))))))))))))
    (:then_1
      (Utilities|IsValid OtherActor
        (:Is%20Valid
          (if (== (Utilities|GetClass OtherActor) "/Game/PlatformTools/Characters/RobotPlayer/Blueprints/BP_PlayerProjectile.BP_PlayerProjectile_C")
            (Variables|Default|SetPlayerCollision false)
            (goto _label)))))))

(event Custom|NME_Loop
  (bind _capsulecomponent (Variables|Collision|GetCapsuleComponent))
  (bind _capsulecomponent_2 (Variables|Collision|GetCapsuleComponent))
  (bind _returnvalue (Transformation|GetWorldLocation _capsulecomponent_2))
  (bind _returnvalue_2 (Transformation|GetWorldLocation _capsulecomponent))
  ;[0 1 0] Main Loop for Enemy Animation
  ;;[0 1 0] Update Mask Flipbook Animation
  (bind _value (Timeline|Flipbook_Timeline PlayFromStart)
    (:Update
      (Rendering|Material|SetScalarParameterValue (Variables|Default|GetDMI_RobotMask) "Anim" _value :!class /Script/Engine.MaterialInstanceDynamic)
      (if (Variables|Default|GetForward)
        ;;[1 1 0] Move Right, Towards Enemy End Location
        (if (< (.x _returnvalue_2) (.x (Variables|Default|GetEndLocation)))
          (Transformation|SetWorldLocationAndRotation _capsulecomponent (Math|Vector|MakeVector (+ (.x _returnvalue_2) (Variables|Default|GetEnemySpeed)) 0.0 (.z _returnvalue_2)) (Math|Rotator|MakeRotator 0.0 0.0 -9e+01) false false)
          (else
            (Variables|Default|SetForward (not (Variables|Default|GetForward)))))
        (else
          ;;[1 0 1] Move Left, Towards Enemy Start Location
          (if (> (.x _returnvalue) (.x (Variables|Default|GetStartLocation)))
            (Transformation|SetWorldLocationAndRotation _capsulecomponent_2 (Math|Vector|MakeVector (- (.x _returnvalue) (Variables|Default|GetEnemySpeed)) 0.0 (.z _returnvalue)) (Math|Rotator|MakeRotator 0.0 0.0 9e+01) false false)
            (else
              (Variables|Default|SetForward (not (Variables|Default|GetForward))))))))
    (:Finished
      (CallFunction|NMELoop))))

(event Custom|ResetDamage
  (bind _bpplatformercomponent (Variables|Default|GetBPPlatformerComponent))
  ;[0 1 0] Player or Projectile Collision with Enemy
  (Utilities|FlowControl|DoOnce false) ; enters at Reset
)

(event EventBeginPlay
  (bind _returnvalue (Game|GetPlayerCharacter 0))
  (bind _returnvalue_2 (Actor|GetComponentbyClass _returnvalue "/Game/PlatformTools/GameDefinitions/Components/BP_Platformer_Main.BP_Platformer_Main_C"))
  ;[0 1 0] Setup Link to Player Component
  (Utilities|FlowControl|Delay 0.2)
  (Utilities|IsValid _returnvalue_2
    (:Is%20Valid
      (Variables|Default|SetBPPlatformerComponent _returnvalue_2)
      ;[1 1 0] Set up Damage Multiplier based on Player Level
      (bind _asgame_instance_platformer (Utilities|Casting|CastToGameInstance_Platformer (Game|GetGameInstance)))
      (Utilities|IsValid _asgame_instance_platformer
        (:Is%20Valid
          (Variables|Default|SetDamageMultiplier (+ (.Skill_Attack_Base (Utilities|Struct|BreakStruct_Characters (Utilities|Array|Get(acopy) (Variables|/Game/PlatformTools/GameDefinitions/GameInstance_Platformer.GameInstance_Platformer_C|GetCharacter _asgame_instance_platformer) (Math|Conversions|ToInteger(Byte) (Variables|/Game/PlatformTools/GameDefinitions/GameInstance_Platformer.GameInstance_Platformer_C|GetPlayerClass _asgame_instance_platformer))))) (* (.PlayerLevel (Utilities|Struct|BreakStruct_Characters (Utilities|Array|Get(acopy) (Variables|/Game/PlatformTools/GameDefinitions/GameInstance_Platformer.GameInstance_Platformer_C|GetCharacter _asgame_instance_platformer) (Math|Conversions|ToInteger(Byte) (Variables|/Game/PlatformTools/GameDefinitions/GameInstance_Platformer.GameInstance_Platformer_C|GetPlayerClass _asgame_instance_platformer))))) (.Skill_Attack_Multiplier (Utilities|Struct|BreakStruct_Characters (Utilities|Array|Get(acopy) (Variables|/Game/PlatformTools/GameDefinitions/GameInstance_Platformer.GameInstance_Platformer_C|GetCharacter _asgame_instance_platformer) (Math|Conversions|ToInteger(Byte) (Variables|/Game/PlatformTools/GameDefinitions/GameInstance_Platformer.GameInstance_Platformer_C|GetPlayerClass _asgame_instance_platformer))))))))
          ;[0 1 0] Main Loop
          (CallFunction|NMELoop))))))

(event Game|Damage|EventAnyDamage
  (params (Damage :type Float%20%28single-precision%29) (DamageType :type Damage%20Type%20Object%20Reference) (InstigatedBy :type Controller%20Object%20Reference) (DamageCauser :type Actor%20Object%20Reference))
  ;[1 0 0] Deal Damage to Enemy
  (bind _output_get (Variables|Default|SetHealth (- (Variables|Default|GetHealth) Damage)))
  (if (<= _output_get 0.0)
    (Utilities|FlowControl|DoOnce false
      (:Completed
        (Rendering|SetVisibility (Variables|Character|GetMesh) false true)
        (Components|Movement|StopMovementImmediately (Variables|Character|GetCharacterMovement))
        (Collision|SetCollisionEnabled (Variables|Collision|GetCapsuleComponent) "NoCollision")
        (Rendering|SetVisibility (Variables|Default|GetParticleSystem) true false)
        (Components|Activation|Activate (Variables|Default|GetParticleSystem) false)
        (Default|ProcessGoals (Variables|Default|GetBPPlatformerComponent) "NewEnumerator2" 1.0)
        (Utilities|FlowControl|Delay 1.0)
        (Actor|DestroyActor)))))

(fn ConstructionScript
  (bind _enddistance (Variables|Default|GetEndDistance))
  (bind _capsulecomponent (Variables|Collision|GetCapsuleComponent))
  (bind _height (Variables|Default|GetHeight))
  (bind _capsulecomponent_2 (Variables|Collision|GetCapsuleComponent))
  (bind _startdistance (Variables|Default|GetStartDistance))
  (bind _height_2 (Variables|Default|GetHeight))
  (bind _capsulecomponent_3 (Variables|Collision|GetCapsuleComponent))
  (bind _returnvalue (Transformation|GetWorldLocation _capsulecomponent_3))
  (bind _returnvalue_2 (Transformation|GetWorldLocation _capsulecomponent))
  (bind _returnvalue_3 (Transformation|GetWorldLocation _capsulecomponent_2))
  (bind _returnvalue_4 (+ (.z _returnvalue_2) _height))
  (bind _returnvalue_5 (+ (.z _returnvalue_3) _height_2))
  (bind _returnvalue_6 (+ (.x _returnvalue_2) _enddistance))
  (bind _returnvalue_7 (+ (.x _returnvalue_3) _startdistance))
  (bind _returnvalue_8 (Math|Vector|MakeVector _returnvalue_6 (.y _returnvalue_2) _returnvalue_4))
  (bind _returnvalue_9 (Math|Vector|MakeVector _returnvalue_7 (.y _returnvalue_3) _returnvalue_5))
  (Utilities|FlowControl|Sequence
    (:then_0
      (if (Variables|Default|GetLockY)
        ;[1 0 0] Lock Y at 0
        (Transformation|SetWorldLocation (Variables|Collision|GetCapsuleComponent) (Math|Vector|MakeVector (.x _returnvalue) 0.0 (.z _returnvalue)) false false)))
    (:then_1
      ;[0 1 0] Setup Dynamic Materials and Flipbook
      (bind _returnvalue_10 (Rendering|Material|CreateDynamicMaterialInstance (Variables|Character|GetMesh) 1 "/Game/PlatformTools/Characters/RobotPlayer/Materials/MI_Robot_Mask.MI_Robot_Mask" "None" :!class /Script/Engine.PrimitiveComponent))
      (bind _output_get (Variables|Default|SetDMI_RobotMask _returnvalue_10))
      (Rendering|Material|SetTextureParameterValue _output_get "FlipbookTexture" (Variables|Appearance|GetFlipbookTexture))
      (Rendering|Material|SetVectorParameterValue _output_get "Color" (Variables|Appearance|GetFlipbookTextureColor) :!class /Script/Engine.MaterialInstanceDynamic)
      (bind _returnvalue_11 (Rendering|Material|CreateDynamicMaterialInstance "/Game/PlatformTools/Characters/RobotPlayer/Materials/MI_Shield.MI_Shield" "None" :!class /Script/Engine.KismetMaterialLibrary))
      (bind _output_get_2 (Variables|Default|SetDMI_Damage _returnvalue_11))
      (Rendering|Material|SetVectorParameterValue _output_get_2 "ShieldColorDark" (Variables|Appearance|GetDamageColorDark) :!class /Script/Engine.MaterialInstanceDynamic)
      (Rendering|Material|SetVectorParameterValue _output_get_2 "ShieldColorDark" (Variables|Appearance|GetDamageColorLight) :!class /Script/Engine.MaterialInstanceDynamic)
      (Rendering|Material|SetScalarParameterValue _output_get_2 "TextureScale" 16.0 :!class /Script/Engine.MaterialInstanceDynamic)
      (Rendering|Material|SetScalarParameterValue _output_get_2 "EmissiveStrength" 1e+01 :!class /Script/Engine.MaterialInstanceDynamic)
      (bind _returnvalue_12 (Rendering|Material|CreateDynamicMaterialInstance (Variables|Character|GetMesh) 0 "/Game/PlatformTools/Characters/RobotEnemy/Materials/MI_Robot_EnemyBody.MI_Robot_EnemyBody" "None" :!class /Script/Engine.PrimitiveComponent))
      (bind _output_get_3 (Variables|Default|SetDMI_RobotBody _returnvalue_12))
      (Rendering|Material|SetVectorParameterValue _output_get_3 "BaseColorG" (Variables|Appearance|GetRobotBodyColor) :!class /Script/Engine.MaterialInstanceDynamic)
      (Rendering|Material|SetVectorParameterValue _output_get_3 "BaseColorB" (Variables|Appearance|GetRobotJointColor) :!class /Script/Engine.MaterialInstanceDynamic)
      (Rendering|Material|SetVectorParameterValue _output_get_3 "BaseColorR" (Variables|Appearance|GetRobotWheelColor) :!class /Script/Engine.MaterialInstanceDynamic)
      ;[1 0 0] Save Robot Body Material (this gets swapped on damage)
      (Variables|Default|SetMI_Slot0 (Rendering|Material|GetMaterial (Variables|Character|GetMesh) 0))
      ;[1 1 0] Set Render Text Above Robot
      (Rendering|Components|TextRender|SetText (Variables|Default|GetTextRender) (Utilities|Text|ToText(String) (Utilities|GetDisplayName self))))
    (:then_2
      ;[1 0 0] Calculate the Enemy Start Position
      (bind _outhit (Collision|LineTraceForObjects _returnvalue_9 (- _returnvalue_9 (Math|Vector|MakeVector 0.0 0.0 (* _height_2 2.0))) (Utilities|Array|MakeArray "ObjectTypeQuery1") false 0 "None"))
      (Variables|Default|SetStartLocation (.impactpoint _outhit))
      (bind _returnvalue_13 (AddComponent|AddChildActorComponent false))
      (Variables|Default|SetEnemy_Start _returnvalue_13)
      (Transformation|SetWorldLocation _returnvalue_13 (.impactpoint _outhit) false false)
      (bind _asbp_enemy_locn (Utilities|Casting|CastToBP_Enemy_Locn (Variables|/Script/Engine.ChildActorComponent|GetChildActor _returnvalue_13)))
      (Variables|/Game/PlatformTools/Characters/RobotEnemy/Blueprints/BP_Enemy_Locn.BP_Enemy_Locn_C|SetText _asbp_enemy_locn (Utilities|Text|ToText(String) (Utilities|GetDisplayName self)))
      (Default|Construction _asbp_enemy_locn))
    (:then_3
      ;[0 0 1] Calculate the Enemy End Position
      (bind _outhit_2 (Collision|LineTraceForObjects _returnvalue_8 (- _returnvalue_8 (Math|Vector|MakeVector 0.0 0.0 (* _height 2.0))) (Utilities|Array|MakeArray "ObjectTypeQuery1") false 0 "None"))
      (Variables|Default|SetEndLocation (.impactpoint _outhit_2))
      (bind _returnvalue_14 (AddComponent|AddChildActorComponent false))
      (Variables|Default|SetEnemy_End _returnvalue_14)
      (Transformation|SetWorldLocation _returnvalue_14 (.impactpoint _outhit_2) false false)
      (bind _asbp_enemy_locn_2 (Utilities|Casting|CastToBP_Enemy_Locn (Variables|/Script/Engine.ChildActorComponent|GetChildActor _returnvalue_14)))
      (Variables|/Game/PlatformTools/Characters/RobotEnemy/Blueprints/BP_Enemy_Locn.BP_Enemy_Locn_C|SetText _asbp_enemy_locn_2 (Utilities|Text|ToText(String) (Utilities|GetDisplayName self)))
      (Default|Construction _asbp_enemy_locn_2))
    (:then_4
      ;[0 1 0] Set Default Rotation towards Enemy Start
      (if (>= (.x (Transformation|GetWorldLocation (Variables|Default|GetEnemy_Start))) (.x (Transformation|GetWorldLocation (Variables|Collision|GetCapsuleComponent))))
        (Transformation|SetWorldRotation (Variables|Collision|GetCapsuleComponent) "0,-90.000000, 0" false false)
        (else
          (Transformation|SetWorldRotation (Variables|Collision|GetCapsuleComponent) "0,90.000000, 0" false false))))))

(fn FacePlayer
  ;[0 1 0] Determine Player Location relative to Enemy and set Forward to move towards that direction
  (Variables|Default|SetForward (> (.x (Transformation|GetWorldLocation (Variables|/Script/Engine.Character|GetMesh (Game|GetPlayerCharacter 0)))) (.x (Transformation|GetWorldLocation (Variables|Character|GetMesh))))))