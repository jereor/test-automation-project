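; Robot player character for a platformer that hands its controls to PlatformerMain and animates its face mask.
; Move, jump and attack inputs, plus first-finger touches for swipe support, are forwarded to PlatformerMain, with jump and attack identified by action type index.
; A self-restarting delay and timeline loop drives a flipbook parameter on the mesh's second material slot, which must already hold a dynamic material instance.
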(event Custom|EyeAnim
  ;[0 1 0] Robot Mask Animation (Gets the Dynamic Material in Slot1 and Updates the Flipbook based on the Timeline)
  (Utilities|FlowControl|Delay 3.0)
  (bind _animpercent (Timeline|RobotMaskAnimTimeline PlayFromStart)
    (:Update
      (bind _asmaterial_instance_dynamic (Utilities|Casting|CastToMaterialInstanceDynamic (Rendering|Material|GetMaterial (Variables|Character|GetMesh) 1)))
      (Utilities|IsValid _asmaterial_instance_dynamic
        (:Is%20Valid
          (Rendering|Material|SetScalarParameterValue _asmaterial_instance_dynamic "Anim" _animpercent :!class /Script/Engine.MaterialInstanceDynamic))))
    (:Finished
      (CallFunction|EyeAnim))))

(event EventBeginPlay
  ;[0 1 0] Start Robot Mask Animation
  (Utilities|FlowControl|Delay 0.2)
  (CallFunction|EyeAnim))

(event Input|ActionEvents|InputActionJump
  (params (Key :type Key%20Structure))
  ;[1 1 0] Replace the default movement controls with this section
  ;;[0 0 1] Replacement Jump Functionality (Action Type - 0)
  (:Pressed
    (Default|CallKeyActionInputPressedEvent (Variables|Default|GetPlatformer_Main)))
  (:Released
    (Default|CallKeyActionInputReleasedEvent (Variables|Default|GetPlatformer_Main))))

(event Input|ActionEvents|InputActionAttack
  (params (Key :type Key%20Structure))
  ;[1 1 0] Replace the default movement controls with this section
  ;;[0 0 1] Replacement Attack Functionality (Action Type - 1)
  (:Pressed
    (Default|CallKeyActionInputPressedEvent (Variables|Default|GetPlatformer_Main) 1))
  (:Released
    (Default|CallKeyActionInputReleasedEvent (Variables|Default|GetPlatformer_Main) 1)))

(event Input|AxisEvents|InputAxisMoveRight
  (params (AxisValue :type Float%20%28single-precision%29))
  ;[1 1 0] Replace the default movement controls with this section
  ;;[0 0 1] Replacement Movement Function
  (Default|CallAxisInputEvent (Variables|Default|GetPlatformer_Main) AxisValue))

(event Input|TouchEvents|InputTouch
  (params (Location :type Vector) (FingerIndex :type ETouchIndex%20Enum))
  (bind _returnvalue (Utilities|Enum|Equal(Enum) FingerIndex "Touch1"))
  ;[1 1 0] Replace the default movement controls with this section
  ;;[1 0 0] Swipe Support Functionality
  (:Pressed
    (if _returnvalue
      (Default|TouchInputEventPressed (Variables|Default|GetPlatformer_Main))))
  (:Released
    (if _returnvalue
      (Default|TouchInputEventReleased (Variables|Default|GetPlatformer_Main)))))

(fn ConstructionScript)