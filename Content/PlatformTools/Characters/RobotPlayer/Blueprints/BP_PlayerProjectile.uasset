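; Player projectile for a side-scrolling character that plays a sound on spawn and flies along X in the player's facing direction.
; A blank Timeline drives updates that trace downward and keep the mesh hovering at a fixed height above the ground.
; Listed ground classes, such as loop splines, destroy it on trace hit.
; Sphere overlaps destroy it after a short delay, except with the player or ignored classes.
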(event OnComponentBeginOverlap(Sphere)
  (params (OverlappedComponent :type Primitive%20Component%20Object%20Reference) (OtherActor :type Actor%20Object%20Reference) (OtherComp :type Primitive%20Component%20Object%20Reference) (OtherBodyIndex :type Integer) (bFromSweep :type Boolean) (SweepResult :type Hit%20Result%20Structure%20%28by%20ref%29))
  ;[1 0 0] Destroy the Projectile if it hits anything. Classes to Ignore will not destroy the projectile if it overlaps the class.
  (Utilities|IsValid OtherActor
    (:Is%20Valid
      (if (and (!= OtherActor (Game|GetPlayerCharacter 0)) (not (Utilities|Array|ContainsItem (Variables|Default|GetClassesToIgnore) (Utilities|GetClass OtherActor))))
        (Utilities|FlowControl|Delay 0.1)
        (Actor|DestroyActor)))))

(event EventBeginPlay
  (bind _staticmesh (Variables|Default|GetStaticMesh))
  (bind _returnvalue (Transformation|GetWorldLocation _staticmesh))
  ;[0 1 0] Fire the Projectile in the direction the player is facing.
  (Audio|PlaySound2D (Variables|Default|GetSoundWave) 1.0 1.0 0.0 0 0)
  (bind _result (Math|Float|NegateFloat (Variables|Default|GetProjectileSpeed))
    (:%20%20
      (Variables|/Script/Engine.MovementComponent|SetVelocity (Variables|Default|GetProjectileMovement) (Math|Vector|MakeVector (* _result (Math|Float|Sign(Float) (.y (Math|Vector|GetForwardVector (Variables|/Script/Engine.Character|GetMesh (Game|GetPlayerCharacter 0)))))) 0.0 0.0))
      ;[1 1 0] Use a blank Timeline to update the Projectile position. Set the position to be 100 units above the ground. Certain ground objects such as loop splines will automatically destroy the projectile.
      (Timeline|Timeline_0 Play
        (:Update
          (bind _outhit (Collision|LineTraceForObjects _returnvalue (+ _returnvalue "0, 0,-500.000000") (Utilities|Array|MakeArray "ObjectTypeQuery1") false 0 "None"))
          (Transformation|SetWorldLocation (Variables|Default|GetStaticMesh) (+ (.impactpoint _outhit) "0, 0,100.000000") false false)
          (if (Utilities|Array|ContainsItem (Variables|Default|GetDestroyProjectileIfHit) (Utilities|GetClass (.hitactor _outhit)))
            (Actor|DestroyActor)))))))

(fn ConstructionScript)