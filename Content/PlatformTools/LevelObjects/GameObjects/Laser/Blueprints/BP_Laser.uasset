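; BP_Laser is a laser hazard that electrocutes the player on contact.
; Its construction script optionally locks Y and fits the endpoints, beam cylinder, trigger box and particles to Width.
; On player overlap it plays a sound, applies damage and disables input through the player's BP_Platformer_Main component.
; It also suspends the character at the impact point without gravity or velocity and lerps the camera to a zoom position via timeline.
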(event OnComponentBeginOverlap(Box)
  (params (OverlappedComponent :type Primitive%20Component%20Object%20Reference) (OtherActor :type Actor%20Object%20Reference) (OtherComp :type Primitive%20Component%20Object%20Reference) (OtherBodyIndex :type Integer) (bFromSweep :type Boolean) (SweepResult :type Hit%20Result%20Structure%20%28by%20ref%29))
  (bind _returnvalue (Game|GetPlayerCharacter 0))
  (bind _bpplatformercomponent (Variables|Default|GetBPPlatformerComponent))
  (bind _charactermovement (Variables|/Script/Engine.Character|GetCharacterMovement _returnvalue))
  ;[0 1 0] Handle Overlap of the Player. Stops Player Movement and Holds In Air. Plays the Electrocute Animation.
  (if (== OtherActor (Game|GetPlayerCharacter 0))
    (Audio|PlaySound2D (Variables|Default|GetSoundWave) 1.0 1.0 0.0 0 0)
    (Default|ApplyPlayerDamage _bpplatformercomponent 1e+02)
    (Variables|/Game/PlatformTools/GameDefinitions/Components/BP_Platformer_Main.BP_Platformer_Main_C|SetIgnoreInputs _bpplatformercomponent true)
    (Transformation|SetWorldLocation (Variables|/Script/Engine.Character|GetCapsuleComponent _returnvalue) (+ (.ImpactPoint (Collision|BreakHitResult SweepResult)) "0, 0,-50.000000") false true)
    (Transformation|SetWorldRotation (Variables|/Script/Engine.Character|GetMesh _returnvalue) "0, 0, 0" false false)
    (Variables|/Script/Engine.CharacterMovementComponent|SetGravityScale _charactermovement 0.0)
    (Variables|/Script/Engine.MovementComponent|SetVelocity _charactermovement "0, 0, 0")
    (bind _output_get (Variables|Default|SetStartZoom (Variables|/Script/Engine.SceneComponent|GetRelativeLocation (Utilities|Array|Get(acopy) (Actor|GetComponentsByClass (Game|GetPlayerCharacter 0) "/Script/Engine.CameraComponent")))))
    (if (Math|Vector|NotEqual(Vector) _output_get (Variables|Default|GetEndZoom) 0.0001)
      (bind _fade (Timeline|Timeline_0 PlayFromStart)
        (:Update
          (Transformation|SetRelativeLocation (Utilities|Array|Get(acopy) (Actor|GetComponentsByClass (Game|GetPlayerCharacter 0) "/Script/Engine.CameraComponent")) (Math|Vector|Lerp(Vector) (Variables|Default|GetStartZoom) (Variables|Default|GetEndZoom) _fade) false false))))))

(event EventBeginPlay
  (bind _returnvalue (Game|GetPlayerCharacter 0))
  (bind _returnvalue_2 (Actor|GetComponentbyClass _returnvalue "/Game/PlatformTools/GameDefinitions/Components/BP_Platformer_Main.BP_Platformer_Main_C"))
  ;[1 1 0] Connect to Platformer_Main Component in Player
  (Utilities|FlowControl|Delay 0.2)
  (Utilities|IsValid _returnvalue_2
    (:Is%20Valid
      (Variables|Default|SetBPPlatformerComponent _returnvalue_2))))

(fn ConstructionScript
  (bind _scene (Variables|Default|GetScene))
  (bind _returnvalue (Transformation|GetWorldLocation _scene))
  (Utilities|FlowControl|Sequence
    (:then_0
      (if (Variables|Default|GetLockY)
        ;[1 0 0] Lock Y at 0
        (Transformation|SetWorldLocation (Variables|Default|GetScene) (Math|Vector|MakeVector (.x _returnvalue) 0.0 (.z _returnvalue)) false false)))
    (:then_1
      ;[0 1 0] Set Start and End of the Laser and Scales
      (bind _result (Math|Float|NegateFloat (/ (Variables|Default|GetWidth) 2.0))
        (:%20%20
          (Transformation|SetRelativeLocation (Variables|Default|GetStart) (Math|Vector|MakeVector _result 0.0 0.0) false false)
          (Transformation|SetRelativeLocation (Variables|Default|GetEnd) (Math|Vector|MakeVector (/ (Variables|Default|GetWidth) 2.0) 0.0 0.0) false false)
          (Transformation|SetWorldScale3D (Variables|Default|GetCylinder) (Math|Vector|MakeVector 0.025 0.025 (/ (Variables|Default|GetWidth) 1e+02)))
          (Transformation|SetWorldScale3D (Variables|Default|GetBox) (Math|Vector|MakeVector (/ (Variables|Default|GetWidth) 5e+01) 1.0 1.0))
          (Transformation|SetWorldScale3D (Variables|Default|GetParticleSystem) (Math|Vector|MakeVector (/ (Variables|Default|GetWidth) 1.1e+03) 0.2 0.2)))))))