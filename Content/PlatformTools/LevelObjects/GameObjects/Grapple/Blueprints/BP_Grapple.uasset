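; Grapple point for a platformer that launches the player on a rope when jump is pressed inside its zone.
; Overlaps set the zone state and grapple reference on the player's BP_Platformer_Main component, whose jump event triggers StartGrapple.
; StartGrapple pauses movement, attaches a temporary CableActor and launches the character left or right by mesh facing.
; The construction script optionally locks Y, previews both launch arcs and configures dynamic materials.
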(event OnComponentBeginOverlap(GrappleZoneCollision)
  (params (OverlappedComponent :type Primitive%20Component%20Object%20Reference) (OtherActor :type Actor%20Object%20Reference) (OtherComp :type Primitive%20Component%20Object%20Reference) (OtherBodyIndex :type Integer) (bFromSweep :type Boolean) (SweepResult :type Hit%20Result%20Structure%20%28by%20ref%29))
  (bind _bpplatformercomponent (Variables|Default|GetBPPlatformerComponent))
  ;[0 1 0] Set %Grapple Zone% in Player Component when overlapped
  (if (== OtherActor (Game|GetPlayerCharacter 0))
    (Variables|/Game/PlatformTools/GameDefinitions/Components/BP_Platformer_Main.BP_Platformer_Main_C|SetGrappleZone _bpplatformercomponent true)
    (Variables|/Game/PlatformTools/GameDefinitions/Components/BP_Platformer_Main.BP_Platformer_Main_C|SetGrappleRef _bpplatformercomponent self)))

(event OnComponentEndOverlap(GrappleZoneCollision)
  (params (OverlappedComponent :type Primitive%20Component%20Object%20Reference) (OtherActor :type Actor%20Object%20Reference) (OtherComp :type Primitive%20Component%20Object%20Reference) (OtherBodyIndex :type Integer))
  (bind _bpplatformercomponent (Variables|Default|GetBPPlatformerComponent))
  ;[1 0 0] Clear %Grapple Zone% in Player Component When Outside the Grapple Zone
  (if (== OtherActor (Game|GetPlayerCharacter 0))
    (Variables|/Game/PlatformTools/GameDefinitions/Components/BP_Platformer_Main.BP_Platformer_Main_C|SetGrappleZone _bpplatformercomponent false)
    (Variables|/Game/PlatformTools/GameDefinitions/Components/BP_Platformer_Main.BP_Platformer_Main_C|SetGrappleRef _bpplatformercomponent self)))

(event Custom|GrappleJump
  ;[1 1 0] Setup Callback to StartGrapple Event
  (CallFunction|StartGrapple))

(event Custom|StartGrapple
  (bind _rightlaunchvelocity (Variables|Default|GetRightLaunchVelocity))
  (bind _leftlaunchvelocity (Variables|Default|GetLeftLaunchVelocity))
  ;[0 1 0] Setup the Grapple When Jump is Pressed in the Grapple Zone - Connect the Rope and Launch the Player
  (Variables|/Game/PlatformTools/GameDefinitions/Components/BP_Platformer_Main.BP_Platformer_Main_C|SetAllowMovement (Variables|Default|GetBPPlatformerComponent) false)
  (Variables|/Game/PlatformTools/GameDefinitions/Components/BP_Platformer_Main.BP_Platformer_Main_C|SetGrappleZone (Variables|Default|GetBPPlatformerComponent) false)
  (CallFunction|AttachCable)
  (Utilities|FlowControl|Delay 0.25)
  (Rendering|SetVisibility (Variables|/Script/CableComponent.CableActor|GetCableComponent (Variables|Default|GetCableRef)) true false)
  (if (< (Math|Float|Sign(Float) (.y (Math|Vector|GetForwardVector (Variables|/Script/Engine.Character|GetMesh (Game|GetPlayerCharacter 0))))) 0.0)
    (if (== (.x (Variables|Default|GetRightLaunchVelocity)) 0.0)
      (Character|LaunchCharacter (Game|GetPlayerCharacter 0) _rightlaunchvelocity false true)
      (else
        (Character|LaunchCharacter (Game|GetPlayerCharacter 0) _rightlaunchvelocity true true)))
    (elif (== (.x (Variables|Default|GetLeftLaunchVelocity)) 0.0)
      (Character|LaunchCharacter (Game|GetPlayerCharacter 0) _leftlaunchvelocity false true)
      (else
        (Character|LaunchCharacter (Game|GetPlayerCharacter 0) _leftlaunchvelocity true true))))
  (Utilities|FlowControl|Delay 1.0)
  (Actor|DestroyActor (Variables|Default|GetCableRef))
  (Variables|/Game/PlatformTools/GameDefinitions/Components/BP_Platformer_Main.BP_Platformer_Main_C|SetAllowMovement (Variables|Default|GetBPPlatformerComponent) true))

(event EventBeginPlay
  (bind _returnvalue (Game|GetPlayerCharacter 0))
  (bind _returnvalue_2 (Actor|GetComponentbyClass _returnvalue "/Game/PlatformTools/GameDefinitions/Components/BP_Platformer_Main.BP_Platformer_Main_C"))
  ;[1 1 0] Connect to Platformer_Main Component in Player
  (Utilities|FlowControl|Delay 0.2)
  (Utilities|IsValid _returnvalue_2
    (:Is%20Valid
      (Variables|Default|SetBPPlatformerComponent _returnvalue_2)
      ;[1 1 0] Setup Callback to StartGrapple Event
      (EventDispatchers|BindEventtoJumpPressedinGrappleZoneEvent (delegate Custom|GrappleJump)))))

(fn ConstructionScript
  (bind _array (Utilities|Array|MakeArray "ObjectTypeQuery3"))
  (bind _grapple_zone_pattern_scale (Variables|Design|GetGrapple%20Zone%20Pattern%20Scale))
  (bind _grapple_zone_pattern_offset (Variables|Design|GetGrapple%20Zone%20Pattern%20Offset))
  (bind _scene (Variables|Default|GetScene))
  (bind _grapple_zone_texture_scale (Variables|Design|GetGrapple%20Zone%20Texture%20Scale))
  (bind _returnvalue (Transformation|GetWorldLocation _scene))
  (Utilities|FlowControl|Sequence
    (:then_0
      (if (Variables|Default|GetLockY)
        ;[1 0 0] Lock Y at 0
        (Transformation|SetWorldLocation (Variables|Default|GetScene) (Math|Vector|MakeVector (.x _returnvalue) 0.0 (.z _returnvalue)) false false)))
    (:then_1
      ;[0 1 0] Show Predicted Path of Grapple in Each Direction
      (Transformation|SetRelativeLocation (Variables|Default|GetGrapple) (Variables|Default|GetGrapplePosition) false false)
      (Class|GameplayStatics|BlueprintPredictProjectilePathbyObjectType (Transformation|GetWorldLocation (Variables|Default|GetScene)) (Variables|Default|GetRightLaunchVelocity) true 0.0 _array false 0 "ForOneFrame")
      (Class|GameplayStatics|BlueprintPredictProjectilePathbyObjectType "0, 0, 0" (Variables|Default|GetLeftLaunchVelocity) true 0.0 _array false 0 "ForOneFrame"))
    (:then_2
      ;[0 1 0] Set Up Dynamic Materials, Colors, Patterns and Scale
      (bind _returnvalue_2 (Rendering|Material|CreateDynamicMaterialInstance (Variables|Default|GetGrapple) 0 "/Game/PlatformTools/LevelObjects/GameObjects/Grapple/Materials/MI_Grapple.MI_Grapple" "DMI_Grapple" :!class /Script/Engine.PrimitiveComponent))
      (Variables|Default|SetDMI_Grapple _returnvalue_2)
      (bind _returnvalue_3 (Rendering|Material|CreateDynamicMaterialInstance (Variables|Default|GetGrappleZone_Plane) 0 "/Game/PlatformTools/LevelObjects/GameObjects/Grapple/Materials/MI_GrappleZonePattern.MI_GrappleZonePattern" "None" :!class /Script/Engine.PrimitiveComponent))
      (Variables|Default|SetDMI_GrappleZone _returnvalue_3)
      (Rendering|Material|SetVectorParameterValue (Variables|Default|GetDMI_GrappleZone) "BaseColorR" (Variables|Design|GetGrappleZone%20Color%20%28R%29) :!class /Script/Engine.MaterialInstanceDynamic)
      (Rendering|Material|SetVectorParameterValue (Variables|Default|GetDMI_GrappleZone) "BaseColorG" (Variables|Design|GetGrappleZone%20Color%20%28G%29) :!class /Script/Engine.MaterialInstanceDynamic)
      (Rendering|Material|SetVectorParameterValue (Variables|Default|GetDMI_GrappleZone) "BaseColorB" (Variables|Design|GetGrappleZone%20Color%20%28B%29) :!class /Script/Engine.MaterialInstanceDynamic)
      (Rendering|Material|SetVectorParameterValue (Variables|Default|GetDMI_Grapple) "BaseColorR" (Variables|Design|GetGrapple%20Color%20-%20Middle%20Circle%20%28R%29) :!class /Script/Engine.MaterialInstanceDynamic)
      (Rendering|Material|SetVectorParameterValue (Variables|Default|GetDMI_Grapple) "BaseColorG" (Variables|Design|GetGrapple%20Color%20-%20Coil%20%28G%29) :!class /Script/Engine.MaterialInstanceDynamic)
      (Rendering|Material|SetVectorParameterValue (Variables|Default|GetDMI_Grapple) "BaseColorB" (Variables|Design|GetGrapple%20Color%20-%20Outer/Inner%20Circle%20%28B%29) :!class /Script/Engine.MaterialInstanceDynamic)
      (Rendering|Material|SetTextureParameterValue (Variables|Default|GetDMI_GrappleZone) "MaterialTexture" (Variables|Design|GetGrapple%20Zone%20Texture))
      (Rendering|Material|SetTextureParameterValue (Variables|Default|GetDMI_GrappleZone) "PatternTexture" (Variables|Design|GetGrapple%20Zone%20Pattern%20Texture))
      (Rendering|Material|SetVectorParameterValue (Variables|Default|GetDMI_GrappleZone) "PatternScale" (Utilities|Struct|MakeLinearColor (.x _grapple_zone_pattern_scale) (.y _grapple_zone_pattern_scale) 0.0 0.0) :!class /Script/Engine.MaterialInstanceDynamic)
      (Rendering|Material|SetVectorParameterValue (Variables|Default|GetDMI_GrappleZone) "PatternOffset" (Utilities|Struct|MakeLinearColor (.x _grapple_zone_pattern_offset) (.y _grapple_zone_pattern_offset) 0.0 0.0) :!class /Script/Engine.MaterialInstanceDynamic)
      (Transformation|SetRelativeScale3D (Variables|Default|GetGrappleZone_Plane) (Math|Vector|MakeVector (.x _grapple_zone_texture_scale) (.y _grapple_zone_texture_scale) 1.0))
      (bind _returnvalue_4 (Rendering|Material|CreateDynamicMaterialInstance "/Game/PlatformTools/LevelObjects/GameObjects/Grapple/Materials/MI_Cable.MI_Cable" "None" :!class /Script/Engine.KismetMaterialLibrary))
      (Variables|Default|SetDMI_Cable _returnvalue_4)
      (Rendering|Material|SetVectorParameterValue (Variables|Default|GetDMI_Cable) "BaseColor" (Variables|Design|GetCableColor) :!class /Script/Engine.MaterialInstanceDynamic))))

(fn AttachCable
  ;[0 1 0] Function to Attach the Cable to the Player Character
  (bind _returnvalue (Game|SpawnActorfromClass "/Script/CableComponent.CableActor" (Math|Transform|MakeTransform "0, 0, 0" "0, 0, 0" "1,1,1") "Undefined" 0 0))
  (Variables|Default|SetCableRef _returnvalue)
  (Rendering|SetVisibility (Variables|/Script/CableComponent.CableActor|GetCableComponent _returnvalue) false false)
  (Variables|/Script/CableComponent.CableComponent|SetSolverIterations (Variables|/Script/CableComponent.CableActor|GetCableComponent _returnvalue) 4)
  (Transformation|AttachActorToActor _returnvalue (Game|GetPlayerCharacter 0) "None" "SnapToTarget" "SnapToTarget" "SnapToTarget" true)
  (Class|CableComponent|SetAttachEndto (Variables|/Script/CableComponent.CableActor|GetCableComponent _returnvalue) self "None" "None")
  (Variables|/Script/CableComponent.CableComponent|SetEndLocation (Variables|/Script/CableComponent.CableActor|GetCableComponent _returnvalue) (Variables|Default|GetGrapplePosition))
  (Rendering|Material|SetMaterial (Variables|/Script/CableComponent.CableActor|GetCableComponent _returnvalue) 0 (Variables|Default|GetDMI_Cable)))