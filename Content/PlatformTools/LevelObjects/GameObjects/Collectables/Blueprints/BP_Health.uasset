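; BP_Health is a health collectable in a platformer toolkit that reports a health increase to the player when touched.
; After a short delay, BeginPlay caches the player's BP_Platformer_Main component and starts a timeline that spins the mesh in yaw.
; Player overlap plays a sound, calls that component's power-up event and destroys the pickup.
; The construction script optionally locks Y to zero and tints inside and outside colors through a dynamic material.
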(event OnComponentBeginOverlap(StaticMesh)
  (params (OverlappedComponent :type Primitive%20Component%20Object%20Reference) (OtherActor :type Actor%20Object%20Reference) (OtherComp :type Primitive%20Component%20Object%20Reference) (OtherBodyIndex :type Integer) (bFromSweep :type Boolean) (SweepResult :type Hit%20Result%20Structure%20%28by%20ref%29))
  ;[0 1 0] Handles Overlap of the PowerUp
  (if (== OtherActor (Game|GetPlayerCharacter 0))
    (Utilities|IsValid OtherActor
      (:Is%20Valid
        (Audio|PlaySound2D (Variables|Default|GetSoundWave) 1.0 1.0 0.0 0 0)
        (Default|CallPowerUpEventBeginOverlap (Variables|Default|GetBPPlatformerComponent) (Variables|Default|GetPowerUpValue) "Health" (Variables|Default|GetHealthIncreasePercentage)))
      (:Is%20Not%20Valid
        _))
    (Audio|Components|Audio|Stop (Variables|Default|GetTimeline_0))
    (Actor|DestroyActor)))

(event EventBeginPlay
  (bind _returnvalue (Game|GetPlayerCharacter 0))
  (bind _returnvalue_2 (Actor|GetComponentbyClass _returnvalue "/Game/PlatformTools/GameDefinitions/Components/BP_Platformer_Main.BP_Platformer_Main_C"))
  ;[1 1 0] Connect to Platformer_Main Component in Player
  (Utilities|FlowControl|Delay 0.2)
  (Utilities|IsValid _returnvalue_2
    (:Is%20Valid
      (Variables|Default|SetBPPlatformerComponent _returnvalue_2)
      ;[0 1 0] Timeline for Object Rotation
      (bind _rotation (Timeline|Timeline_0 Play)
        (:Update
          (Utilities|IsValid (Variables|Default|GetStaticMesh)
            (:Is%20Valid
              (Transformation|SetWorldRotation (Variables|Default|GetStaticMesh) (Math|Rotator|MakeRotator 0.0 0.0 _rotation) false false))))))))

(fn ConstructionScript
  (bind _scene (Variables|Default|GetScene))
  (bind _returnvalue (Transformation|GetWorldLocation _scene))
  (Utilities|FlowControl|Sequence
    (:then_0
      (if (Variables|Default|GetLockY)
        ;[1 0 0] Lock Y at 0
        (Transformation|SetWorldLocation (Variables|Default|GetScene) (Math|Vector|MakeVector (.x _returnvalue) 0.0 (.z _returnvalue)) false false)))
    (:then_1
      ;[0 1 0] Setup Dynamic Material Instances
      (bind _returnvalue_2 (Rendering|Material|CreateDynamicMaterialInstance (Variables|Default|GetStaticMesh) 0 "/Game/PlatformTools/LevelObjects/GameObjects/Collectables/Materials/MI_Unllit_RGB.MI_Unllit_RGB" "None" :!class /Script/Engine.PrimitiveComponent))
      (bind _output_get (Variables|Default|SetColorDMI _returnvalue_2))
      (Rendering|Material|SetVectorParameterValue _output_get "BaseColorR" (Variables|Design|GetOutsideColor) :!class /Script/Engine.MaterialInstanceDynamic)
      (Rendering|Material|SetVectorParameterValue _output_get "BaseColorG" (Variables|Design|GetInsideColor) :!class /Script/Engine.MaterialInstanceDynamic))))