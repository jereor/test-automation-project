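; BP_Cannon is a platformer level hazard that repeatedly fires spiked cannonballs on a fixed delay.
; Once it finds the player's BP_Platformer_Main component, each shot plays an animation and spawns a BP_SpikedBall with limited lifetime, flipping its X velocity when FacingRight.
; An overlap volume tracks the player, who takes damage directly at firing time if inside.
; The Construction Script optionally locks Y to zero, applies facing, tints a dynamic material and sets a name label.
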(event OnComponentBeginOverlap(PlayerDetection)
  (params (OverlappedComponent :type Primitive%20Component%20Object%20Reference) (OtherActor :type Actor%20Object%20Reference) (OtherComp :type Primitive%20Component%20Object%20Reference) (OtherBodyIndex :type Integer) (bFromSweep :type Boolean) (SweepResult :type Hit%20Result%20Structure%20%28by%20ref%29))
  ;[1 0 0] Detect Player in front of Cannon
  (if (== OtherActor (Game|GetPlayerCharacter 0))
    (Variables|Default|SetPlayerDetected true)))

(event OnComponentEndOverlap(PlayerDetection)
  (params (OverlappedComponent :type Primitive%20Component%20Object%20Reference) (OtherActor :type Actor%20Object%20Reference) (OtherComp :type Primitive%20Component%20Object%20Reference) (OtherBodyIndex :type Integer))
  ;[0 1 0] Clear Detected Player if Player Moves Out of Range
  (if (== OtherActor (Game|GetPlayerCharacter 0))
    (Variables|Default|SetPlayerDetected false)))

(event Custom|FireCannon
  (bind _bpplatformercomponent (Variables|Default|GetBPPlatformerComponent))
  ;[0 1 0] Animate the Cannon, Fire the Cannonball, Detect Player Presence
  (Components|Animation|PlayAnimation (Variables|Default|GetCannonMesh) "/Game/PlatformTools/LevelObjects/GameObjects/Cannon/Animations/Cannon.Cannon" false)
  (bind _returnvalue (Game|SpawnActorfromClass "/Game/PlatformTools/LevelObjects/GameObjects/Cannon/ReferencedBP/BP_SpikedBall.BP_SpikedBall_C" (Math|Transform|MakeTransform (Transformation|GetWorldLocation (Variables|Default|GetArrow)) "0, 0, 0" "1,1,1") "Undefined" 0 0))
  (Utilities|IsValid _returnvalue
    (:Is%20Valid
      (Actor|SetLifeSpan _returnvalue (Variables|Default|GetCannonBallLifeTime))
      (Collision|SetCollisionEnabled (Variables|/Game/PlatformTools/LevelObjects/GameObjects/Cannon/ReferencedBP/BP_SpikedBall.BP_SpikedBall_C|GetSphere _returnvalue) "QueryAndPhysics")
      (if (Variables|Default|GetFacingRight)
        (Variables|/Script/Engine.MovementComponent|SetVelocity (Variables|/Game/PlatformTools/LevelObjects/GameObjects/Cannon/ReferencedBP/BP_SpikedBall.BP_SpikedBall_C|GetProjectileMovement _returnvalue) (Math|Vector|MakeVector (* (.x (Variables|/Script/Engine.MovementComponent|GetVelocity (Variables|/Game/PlatformTools/LevelObjects/GameObjects/Cannon/ReferencedBP/BP_SpikedBall.BP_SpikedBall_C|GetProjectileMovement _returnvalue))) -1.0) (.y (Variables|/Script/Engine.MovementComponent|GetVelocity (Variables|/Game/PlatformTools/LevelObjects/GameObjects/Cannon/ReferencedBP/BP_SpikedBall.BP_SpikedBall_C|GetProjectileMovement _returnvalue))) (.z (Variables|/Script/Engine.MovementComponent|GetVelocity (Variables|/Game/PlatformTools/LevelObjects/GameObjects/Cannon/ReferencedBP/BP_SpikedBall.BP_SpikedBall_C|GetProjectileMovement _returnvalue))))))
      ;;[1 1 1] Apply Damage to the Player if he is standing in front of the cannon
      (if (Variables|Default|GetPlayerDetected)
        (Utilities|IsValid _bpplatformercomponent
          (:Is%20Valid
            (Default|CallApplyDamageEvent _bpplatformercomponent 2e+01))))
      (Utilities|FlowControl|Delay 5.0)
      (CallFunction|FireCannon))))

(event EventBeginPlay
  (bind _returnvalue (Game|GetPlayerCharacter 0))
  (bind _returnvalue_2 (Actor|GetComponentbyClass _returnvalue "/Game/PlatformTools/GameDefinitions/Components/BP_Platformer_Main.BP_Platformer_Main_C"))
  ;[1 1 0] Connect to Platformer_Main Component in Player
  (Utilities|FlowControl|Delay 0.2)
  (Utilities|IsValid _returnvalue_2
    (:Is%20Valid
      (Variables|Default|SetBPPlatformerComponent _returnvalue_2)
      (CallFunction|FireCannon))))

(fn ConstructionScript
  (bind _scene (Variables|Default|GetScene))
  (bind _returnvalue (Transformation|GetWorldLocation _scene))
  (Utilities|FlowControl|Sequence
    (:then_0
      (if (Variables|Default|GetLockY)
        ;[1 0 0] Lock Y at 0
        (Transformation|SetWorldLocation (Variables|Default|GetScene) (Math|Vector|MakeVector (.x _returnvalue) 0.0 (.z _returnvalue)) false false)))
    (:then_1
      ;[0 1 0] Setup Material Instances
      (bind _returnvalue_2 (Rendering|Material|CreateDynamicMaterialInstance (Variables|Default|GetCannonMesh) 0 "/Game/PlatformTools/LevelObjects/GameObjects/Cannon/Materials/MI_Cannon.MI_Cannon" "None" :!class /Script/Engine.PrimitiveComponent))
      (bind _output_get (Variables|Default|SetColorDMI _returnvalue_2))
      (Rendering|Material|SetVectorParameterValue _output_get "BaseColorG" (Variables|Design|GetDetailColor) :!class /Script/Engine.MaterialInstanceDynamic)
      (Rendering|Material|SetVectorParameterValue _output_get "BaseColorR" (Variables|Design|GetCannonColor) :!class /Script/Engine.MaterialInstanceDynamic)
      (Rendering|Material|SetVectorParameterValue _output_get "BaseColorB" (Variables|Design|GetWheelColor) :!class /Script/Engine.MaterialInstanceDynamic)
      (if (Variables|Default|GetFacingRight)
        (Transformation|SetWorldRotation (Variables|Default|GetCannonRotation) "0,180.000000, 0" false false))
      (Rendering|Components|TextRender|SetText (Variables|Default|GetTextRender) (Utilities|Text|ToText(String) (Utilities|GetDisplayName self))))))