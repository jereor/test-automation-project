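; BP_SpikedBall is a spiked cannonball hazard that damages the player on contact.
; Shortly after BeginPlay it caches the player's BP_Platformer_Main component.
; The first sphere overlap with the player passes PlayerDamage to that component's damage event, then destroys the ball after a brief delay.
; The construction script creates a dynamic material instance to apply configurable ball and spike colors.
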(event OnComponentBeginOverlap(Sphere)
  (params (OverlappedComponent :type Primitive%20Component%20Object%20Reference) (OtherActor :type Actor%20Object%20Reference) (OtherComp :type Primitive%20Component%20Object%20Reference) (OtherBodyIndex :type Integer) (bFromSweep :type Boolean) (SweepResult :type Hit%20Result%20Structure%20%28by%20ref%29))
  ;[0 1 0] Handle Damage on Overlap
  (if (== OtherActor (Game|GetPlayerCharacter 0))
    (Utilities|FlowControl|DoOnce false
      (:Completed
        (Utilities|IsValid (Variables|Default|GetBPPlatformerComponent)
          (:Is%20Valid
            (Default|CallApplyDamageEvent (Variables|Default|GetBPPlatformerComponent) (Variables|Default|GetPlayerDamage)))
          (:Is%20Not%20Valid
            _))
        (Utilities|FlowControl|Delay 0.1)
        (Actor|DestroyActor)))))

(event EventBeginPlay
  (bind _returnvalue (Game|GetPlayerCharacter 0))
  (bind _returnvalue_2 (Actor|GetComponentbyClass _returnvalue "/Game/PlatformTools/GameDefinitions/Components/BP_Platformer_Main.BP_Platformer_Main_C"))
  ;[1 1 0] Connect to Platformer_Main Component in Player
  (Utilities|FlowControl|Delay 0.2)
  (Utilities|IsValid _returnvalue_2
    (:Is%20Valid
      (Variables|Default|SetBPPlatformerComponent _returnvalue_2))))

(fn ConstructionScript
  ;[0 1 0] Set up Dynamic Material Instances
  (bind _returnvalue (Rendering|Material|CreateDynamicMaterialInstance (Variables|Default|GetStaticMesh) 0 "/Game/PlatformTools/LevelObjects/GameObjects/Cannon/Materials/MI_CannonBall.MI_CannonBall" "None" :!class /Script/Engine.PrimitiveComponent))
  (bind _output_get (Variables|Default|SetColorDMI _returnvalue))
  (Rendering|Material|SetVectorParameterValue _output_get "BaseColorB" (Variables|Design|GetCannonBallColor) :!class /Script/Engine.MaterialInstanceDynamic)
  (Rendering|Material|SetVectorParameterValue _output_get "BaseColorR" (Variables|Design|GetSpikeColor) :!class /Script/Engine.MaterialInstanceDynamic))