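; Slime waterfall level object that animates slime flowing along a spline and can push the player.
; The construction script splits the spline into paired, two-layer spline meshes with tinted dynamic materials, optionally locking Y to zero.
; The SlimeMover timeline slides segments one length along the spline, in either direction, to fake flow.
; Box overlap enables a per-update player offset and optionally triggers the platformer component's water events for health effects.
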(event OnComponentBeginOverlap(Box)
  (params (OverlappedComponent :type Primitive%20Component%20Object%20Reference) (OtherActor :type Actor%20Object%20Reference) (OtherComp :type Primitive%20Component%20Object%20Reference) (OtherBodyIndex :type Integer) (bFromSweep :type Boolean) (SweepResult :type Hit%20Result%20Structure%20%28by%20ref%29))
  (bind _bpplatformercomponent (Variables|Default|GetBPPlatformerComponent))
  ;[0 1 0] Handle Player Overlap With Slime (Similar to Water)
  (if (== OtherActor (Game|GetPlayerCharacter 0))
    (Variables|Default|SetMovePlayer? true)
    (if (Variables|Default|GetSlimeAffectsPlayerHealth)
      (Utilities|IsValid _bpplatformercomponent
        (:Is%20Valid
          (Default|CallWaterEventBeginOverlap _bpplatformercomponent))))))

(event OnComponentEndOverlap(Box)
  (params (OverlappedComponent :type Primitive%20Component%20Object%20Reference) (OtherActor :type Actor%20Object%20Reference) (OtherComp :type Primitive%20Component%20Object%20Reference) (OtherBodyIndex :type Integer))
  (bind _bpplatformercomponent (Variables|Default|GetBPPlatformerComponent))
  ;[0 1 0] Handle Player Moving Outside of Slime
  (if (== OtherActor (Game|GetPlayerCharacter 0))
    (Variables|Default|SetMovePlayer? false)
    (if (Variables|Default|GetSlimeAffectsPlayerHealth)
      (Utilities|IsValid _bpplatformercomponent
        (:Is%20Valid
          (Default|CallWaterEventEndOverlap _bpplatformercomponent))))))

(event EventBeginPlay
  (bind _returnvalue (Game|GetPlayerCharacter 0))
  (bind _spline (Variables|Default|GetSpline))
  (bind _spline_2 (Variables|Default|GetSpline))
  (bind _returnvalue_2 (Actor|GetComponentbyClass _returnvalue "/Game/PlatformTools/GameDefinitions/Components/BP_Platformer_Main.BP_Platformer_Main_C"))
  ;[1 1 0] Connect to Platformer_Main Component in Player
  (Utilities|FlowControl|Delay 0.2)
  (Utilities|IsValid _returnvalue_2
    (:Is%20Valid
      (Variables|Default|SetBPPlatformerComponent _returnvalue_2)
      ;[0 1 0] Setup Slime Playback and Direction
      (if (Variables|Default|GetReverse?)
        (Variables|Default|SetLerpA 0.0)
        (Variables|Default|SetLerpB (Variables|Default|GetSlimeLength))
        (else
          (Variables|Default|SetLerpA (Variables|Default|GetSlimeLength))
          (Variables|Default|SetLerpB 0.0)
          (bind _result (Math|Float|NegateFloat (Variables|Default|GetPlayerSpeed))
            (:%20%20
              (Variables|Default|SetPlayerSpeed _result)))))
      (Components|Timeline|SetPlayRate (Variables|Default|GetSlimeMover) (Variables|Default|GetSlimePlaybackSpeed))
      (bind _percentage (Timeline|SlimeMover Play)
        (:Update
          (Utilities|FlowControl|Sequence
            (:then_0
              (for _index (range 0 (- (Variables|Default|GetNumberofSlimeElements) 1))
                (Utilities|IsValid (Utilities|Array|Get(acopy) (Variables|Default|GetSplines) (* _index 2))
                  (:Is%20Valid
                    (SplineMesh|SetStartandEnd (Utilities|Array|Get(acopy) (Variables|Default|GetSplines) (* _index 2)) (Spline|GetLocationatDistanceAlongSpline _spline (+ (* _index (Variables|Default|GetSlimeLength)) (Math|Float|Lerp (Variables|Default|GetLerpA) (Variables|Default|GetLerpB) _percentage)) "World") (Spline|GetTangentatDistanceAlongSpline _spline (+ (* _index (Variables|Default|GetSlimeLength)) (Math|Float|Lerp (Variables|Default|GetLerpA) (Variables|Default|GetLerpB) _percentage)) "World") (Spline|GetLocationatDistanceAlongSpline _spline_2 (+ (* (+ _index 1) (Variables|Default|GetSlimeLength)) (Math|Float|Lerp (Variables|Default|GetLerpA) (Variables|Default|GetLerpB) _percentage)) "World") (Spline|GetTangentatDistanceAlongSpline _spline_2 (+ (* (+ _index 1) (Variables|Default|GetSlimeLength)) (Math|Float|Lerp (Variables|Default|GetLerpA) (Variables|Default|GetLerpB) _percentage)) "World") true :!class /Script/Engine.SplineMeshComponent)
                    (Utilities|IsValid (Utilities|Array|Get(acopy) (Variables|Default|GetSplines) (+ (* _index 2) 1))
                      (:Is%20Valid
                        (SplineMesh|SetStartandEnd (Utilities|Array|Get(acopy) (Variables|Default|GetSplines) (+ (* _index 2) 1)) (Spline|GetLocationatDistanceAlongSpline _spline (+ (* _index (Variables|Default|GetSlimeLength)) (Math|Float|Lerp (Variables|Default|GetLerpA) (Variables|Default|GetLerpB) _percentage)) "World") (Spline|GetTangentatDistanceAlongSpline _spline (+ (* _index (Variables|Default|GetSlimeLength)) (Math|Float|Lerp (Variables|Default|GetLerpA) (Variables|Default|GetLerpB) _percentage)) "World") (Spline|GetLocationatDistanceAlongSpline _spline_2 (+ (* (+ _index 1) (Variables|Default|GetSlimeLength)) (Math|Float|Lerp (Variables|Default|GetLerpA) (Variables|Default|GetLerpB) _percentage)) "World") (Spline|GetTangentatDistanceAlongSpline _spline_2 (+ (* (+ _index 1) (Variables|Default|GetSlimeLength)) (Math|Float|Lerp (Variables|Default|GetLerpA) (Variables|Default|GetLerpB) _percentage)) "World") true :!class /Script/Engine.SplineMeshComponent)))))))
            (:then_1
              (if (Variables|Default|GetMovePlayer?)
                (Transformation|AddActorLocalOffset (Game|GetPlayerCharacter 0) (Math|Vector|MakeVector (* (Variables|Default|GetSlimePlaybackSpeed) (Variables|Default|GetPlayerSpeed)) 0.0 0.0) false false)))))))))

(fn ConstructionScript
  (bind _numberofslimeelements (Variables|Default|GetNumberofSlimeElements))
  (bind _spline (Variables|Default|GetSpline))
  (bind _sceneroot (Variables|Default|GetSceneRoot))
  (bind _returnvalue (Transformation|GetWorldLocation _sceneroot))
  (Utilities|FlowControl|Sequence
    (:then_0
      (if (Variables|Default|GetLockY)
        ;[1 0 0] Lock Y at 0
        (Transformation|SetWorldLocation (Variables|Default|GetSceneRoot) (Math|Vector|MakeVector (.x _returnvalue) 0.0 (.z _returnvalue)) false false)))
    (:then_1
      ;[0 1 0] Setup Colors
      (bind _returnvalue_2 (Rendering|Material|CreateDynamicMaterialInstance "/Game/PlatformTools/LevelObjects/GameObjects/SlimeSplines/Materials/MI_SlimeWaterfall.MI_SlimeWaterfall" "None" :!class /Script/Engine.KismetMaterialLibrary))
      (Variables|Default|SetDMI_SlimeA _returnvalue_2)
      (bind _returnvalue_3 (Rendering|Material|CreateDynamicMaterialInstance "/Game/PlatformTools/LevelObjects/GameObjects/SlimeSplines/Materials/MI_SlimeWaterfall.MI_SlimeWaterfall" "None" :!class /Script/Engine.KismetMaterialLibrary))
      (Variables|Default|SetDMI_SlimeB _returnvalue_3)
      (Rendering|Material|SetVectorParameterValue (Variables|Default|GetDMI_SlimeA) "WaterColor" (Variables|Design|GetColorA) :!class /Script/Engine.MaterialInstanceDynamic)
      (Rendering|Material|SetVectorParameterValue (Variables|Default|GetDMI_SlimeA) "FresnelColor" (Variables|Design|GetFresnelA) :!class /Script/Engine.MaterialInstanceDynamic)
      (Rendering|Material|SetVectorParameterValue (Variables|Default|GetDMI_SlimeB) "WaterColor" (Variables|Design|GetColorB) :!class /Script/Engine.MaterialInstanceDynamic)
      (Rendering|Material|SetVectorParameterValue (Variables|Default|GetDMI_SlimeB) "FresnelColor" (Variables|Design|GetFresnelB) :!class /Script/Engine.MaterialInstanceDynamic)
      (Rendering|Material|SetScalarParameterValue (Variables|Default|GetDMI_SlimeA) "Height" (- (.z (Transformation|GetWorldLocation (Variables|Default|GetSpline))) (Variables|Default|GetWaterfallHeight)) :!class /Script/Engine.MaterialInstanceDynamic))
    (:then_2
      ;[0 1 0] Place Slime Meshes on Spline
      (Utilities|Array|Clear (Variables|Default|GetSplines))
      (Variables|Default|SetSlimeLength (/ (Spline|GetSplineLength (Variables|Default|GetSpline)) (Math|Conversions|ToFloat(Integer) _numberofslimeelements)))
      (for _index (range 0 (- _numberofslimeelements 1))
        (Utilities|FlowControl|Sequence
          (:then_0
            (bind _returnvalue_4 (AddComponent|AddSplineMeshComponent true))
            (SplineMesh|SetStartandEnd _returnvalue_4 (Spline|GetLocationatDistanceAlongSpline _spline (* _index (Variables|Default|GetSlimeLength)) "World") (Spline|GetTangentatDistanceAlongSpline _spline (* _index (Variables|Default|GetSlimeLength)) "World") (Spline|GetLocationatDistanceAlongSpline _spline (* (+ _index 1) (Variables|Default|GetSlimeLength)) "World") (Spline|GetTangentatDistanceAlongSpline _spline (* (+ _index 1) (Variables|Default|GetSlimeLength)) "World") true :!class /Script/Engine.SplineMeshComponent)
            (Components|StaticMesh|SetStaticMesh _returnvalue_4 (Variables|Design|GetSlimeA_Mesh))
            (Rendering|Material|SetMaterial _returnvalue_4 0 (Variables|Default|GetDMI_SlimeA))
            (Utilities|Array|AddUnique (Variables|Default|GetSplines) _returnvalue_4))
          (:then_1
            (bind _returnvalue_5 (AddComponent|AddSplineMeshComponent true (Math|Transform|MakeTransform "0, 0, 0" "0, 0, 0" "1,2.000000,1.000000")))
            (SplineMesh|SetStartandEnd _returnvalue_5 (Spline|GetLocationatDistanceAlongSpline _spline (* _index (Variables|Default|GetSlimeLength)) "World") (Spline|GetTangentatDistanceAlongSpline _spline (* _index (Variables|Default|GetSlimeLength)) "World") (Spline|GetLocationatDistanceAlongSpline _spline (* (+ _index 1) (Variables|Default|GetSlimeLength)) "World") (Spline|GetTangentatDistanceAlongSpline _spline (* (+ _index 1) (Variables|Default|GetSlimeLength)) "World") true :!class /Script/Engine.SplineMeshComponent)
            (Components|StaticMesh|SetStaticMesh _returnvalue_5 (Variables|Design|GetSlimeB_Mesh))
            (Rendering|Material|SetMaterial _returnvalue_5 0 (Variables|Default|GetDMI_SlimeB))
            (Utilities|Array|AddUnique (Variables|Default|GetSplines) _returnvalue_5)))))))