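; BP_Box is a placeable box level object for a platformer, configured entirely in its construction script.
; It can lock its Y position to zero for a side-on plane and creates dynamic edge and pattern materials from exposed color, texture, offset and scale settings.
; With JumpAssist enabled, it attaches a BP_PrecisionJump child actor above itself, overrides both jump directions with a vertical JumpHeight and draws predicted projectile paths for debugging.
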(fn ConstructionScript
  (bind _array (Utilities|Array|MakeArray "ObjectTypeQuery3"))
  (bind _scene (Variables|Default|GetScene))
  (bind _patternoffset (Variables|Design|GetPatternOffset))
  (bind _patternscale (Variables|Design|GetPatternScale))
  (bind _jumpheight (Variables|Default|GetJumpHeight))
  (bind _scene_2 (Variables|Default|GetScene))
  (bind _returnvalue (Transformation|GetWorldLocation _scene_2))
  (bind _returnvalue_2 (Transformation|GetWorldLocation _scene))
  (bind _returnvalue_3 (+ _returnvalue_2 "0, 0,50.000000"))
  (Utilities|FlowControl|Sequence
    (:then_0
      (if (Variables|Default|GetLockY)
        ;[1 0 0] Lock Y at 0
        (Transformation|SetWorldLocation (Variables|Default|GetScene) (Math|Vector|MakeVector (.x _returnvalue) 0.0 (.z _returnvalue)) false false)))
    (:then_1
      ;[0 1 0] Create Dynamic Material Instances
      (bind _returnvalue_4 (Rendering|Material|CreateDynamicMaterialInstance (Variables|Default|GetStaticMesh) 1 "/Game/PlatformTools/LevelObjects/GameObjects/Boxes/Materials/MI_BoxEdge.MI_BoxEdge" "None" :!class /Script/Engine.PrimitiveComponent))
      (Variables|Default|SetBoxEdgeMatInst _returnvalue_4)
      (bind _returnvalue_5 (Rendering|Material|CreateDynamicMaterialInstance (Variables|Default|GetStaticMesh) 0 "/Game/PlatformTools/LevelObjects/GameObjects/Boxes/Materials/MI_BoxPattern.MI_BoxPattern" "None" :!class /Script/Engine.PrimitiveComponent))
      (Variables|Default|SetBoxPatternMatInst _returnvalue_5)
      (Rendering|Material|SetVectorParameterValue (Variables|Default|GetBoxEdgeMatInst) "BaseColor" (Variables|Design|GetEdgeColor) :!class /Script/Engine.MaterialInstanceDynamic)
      (Rendering|Material|SetVectorParameterValue (Variables|Default|GetBoxPatternMatInst) "BaseColor" (Variables|Design|GetPatternColor) :!class /Script/Engine.MaterialInstanceDynamic)
      (Rendering|Material|SetTextureParameterValue (Variables|Default|GetBoxPatternMatInst) "PatternTexture" (Variables|Design|GetPatternTexture))
      (Rendering|Material|SetVectorParameterValue (Variables|Default|GetBoxPatternMatInst) "PatternOffset" (Utilities|Struct|MakeLinearColor (.x _patternoffset) (.y _patternoffset) 0.0 0.0) :!class /Script/Engine.MaterialInstanceDynamic)
      (Rendering|Material|SetVectorParameterValue (Variables|Default|GetBoxPatternMatInst) "PatternScale" (Utilities|Struct|MakeLinearColor (.x _patternscale) (.y _patternscale) 0.0 0.0) :!class /Script/Engine.MaterialInstanceDynamic)
      (if (Variables|Default|GetJumpAssist?)
        ;[1 1 0] Add Precision Jump Component if %JumpAssist?% has been set
        (bind _returnvalue_6 (AddComponent|AddChildActorComponent false (Math|Transform|MakeTransform "0, 0,50.000000" "0, 0, 0" "0.400000,0.400000,0.400000")))
        (ChildActorComponent|SetChildActorClass _returnvalue_6 "/Game/PlatformTools/LevelObjects/HelperObjects/Jumps/Blueprints/BP_PrecisionJump.BP_PrecisionJump_C")
        (Transformation|SetMobility _returnvalue_6 "Static")
        (bind _asbp_precision_jump (Utilities|Casting|CastToBP_PrecisionJump (Variables|/Script/Engine.ChildActorComponent|GetChildActor _returnvalue_6)))
        (Utilities|IsValid (Variables|/Script/Engine.ChildActorComponent|GetChildActor _returnvalue_6)
          (:Is%20Valid
            (Variables|/Game/PlatformTools/LevelObjects/HelperObjects/Jumps/Blueprints/BP_PrecisionJump.BP_PrecisionJump_C|SetJumpRightOverride _asbp_precision_jump (Math|Vector|MakeVector 0.0 0.0 _jumpheight))
            (Variables|/Game/PlatformTools/LevelObjects/HelperObjects/Jumps/Blueprints/BP_PrecisionJump.BP_PrecisionJump_C|SetJumpLeftOverride _asbp_precision_jump (Math|Vector|MakeVector 0.0 0.0 _jumpheight))
            (Class|GameplayStatics|BlueprintPredictProjectilePathbyObjectType _returnvalue_3 "0, 0, 0" true 0.0 _array false 0 "ForOneFrame")
            (Class|GameplayStatics|BlueprintPredictProjectilePathbyObjectType _returnvalue_3 "0, 0, 0" true 0.0 _array false 0 "ForOneFrame")))))))