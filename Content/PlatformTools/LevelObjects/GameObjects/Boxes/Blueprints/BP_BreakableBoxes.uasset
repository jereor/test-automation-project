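; Breakable box stack that explodes after the player touches its trigger, damaging them if they are still inside.
; The first overlap runs a once-only color timeline scaled to PlaybackTime, then swaps the box for a physics-driven BP_SplitBox, drops the barrier collision and releases the top box.
; Damage goes through the player's BP_Platformer_Main component.
; The construction script builds dynamic materials for three boxes and optionally locks world Y to zero.
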(event OnComponentBeginOverlap(Box)
  (params (OverlappedComponent :type Primitive%20Component%20Object%20Reference) (OtherActor :type Actor%20Object%20Reference) (OtherComp :type Primitive%20Component%20Object%20Reference) (OtherBodyIndex :type Integer) (bFromSweep :type Boolean) (SweepResult :type Hit%20Result%20Structure%20%28by%20ref%29))
  ;[0 1 0] Start Color Change Timeline, Explode the Box using Physics, Apply Damage to Player if Standing Too Close
  (if (== OtherActor (Game|GetPlayerCharacter 0))
    (Variables|Default|SetDamagePlayer true)
    (Utilities|FlowControl|DoOnce false
      (:Completed
        (Components|Timeline|SetPlayRate (Variables|Default|GetChangeColor) (/ (Components|Timeline|GetTimelineLength (Variables|Default|GetChangeColor)) (Variables|Default|GetPlayback%20Time)))
        (bind _time (Timeline|ChangeColor PlayFromStart)
          (:Update
            (Rendering|Material|SetVectorParameterValue (Variables|Design_Breakable|GetBreakableBoxEdgeMI) "BaseColor" (Math|Curves|GetLinearColorValue (Variables|Default|GetCurveLinearColor) _time) :!class /Script/Engine.MaterialInstanceDynamic)
            (Rendering|Material|SetVectorParameterValue (Variables|Design_Breakable|GetBreakableBoxPatternMI) "BaseColor" (Math|Curves|GetLinearColorValue (Variables|Default|GetCurveLinearColor) _time) :!class /Script/Engine.MaterialInstanceDynamic))
          (:Finished
            (Components|DestroyComponent (Variables|Default|GetBreakableBox))
            (Collision|SetCollisionEnabled (Variables|Default|GetBarrier) "NoCollision")
            (Rendering|SetVisibility (Variables|Default|GetSplitBox) true false)
            (bind _asbp_split_box (Utilities|Casting|CastToBP_SplitBox (Variables|/Script/Engine.ChildActorComponent|GetChildActor (Variables|Default|GetSplitBox))))
            (Default|EnablePhysics _asbp_split_box)
            (Physics|SetSimulatePhysics (Variables|Default|GetTopBox) true)
            (Audio|PlaySound2D (Variables|Default|GetSoundWave) 1.0 1.0 0.0 0 0)
            (if (Variables|Default|GetDamagePlayer)
              (Default|ApplyPlayerDamage (Variables|Default|GetBPPlatformerComponent) 5e+01))))))))

(event OnComponentEndOverlap(Box)
  (params (OverlappedComponent :type Primitive%20Component%20Object%20Reference) (OtherActor :type Actor%20Object%20Reference) (OtherComp :type Primitive%20Component%20Object%20Reference) (OtherBodyIndex :type Integer))
  ;[0 1 0] Turn off Damage to Player if Player Moves Back Far Enough
  (if (== OtherActor (Game|GetPlayerCharacter 0))
    (Variables|Default|SetDamagePlayer false)))

(event EventBeginPlay
  (bind _returnvalue (Game|GetPlayerCharacter 0))
  (bind _returnvalue_2 (Actor|GetComponentbyClass _returnvalue "/Game/PlatformTools/GameDefinitions/Components/BP_Platformer_Main.BP_Platformer_Main_C"))
  ;[1 1 0] Connect to Platformer_Main Component in Player
  (Utilities|FlowControl|Delay 0.2)
  (Utilities|IsValid _returnvalue_2
    (:Is%20Valid
      (Variables|Default|SetBPPlatformerComponent _returnvalue_2))))

(fn ConstructionScript
  (bind _bottomboxpatternoffset (Variables|Design_BottomBox|GetBottomBoxPatternOffset))
  (bind _bottomboxpatternscale (Variables|Design_BottomBox|GetBottomBoxPatternScale))
  (bind _breakablepatternoffset (Variables|Design_Breakable|GetBreakablePatternOffset))
  (bind _breakablepatternscale (Variables|Design_Breakable|GetBreakablePatternScale))
  (bind _scene (Variables|Default|GetScene))
  (bind _topboxpatternoffset (Variables|Design_TopBox|GetTopBoxPatternOffset))
  (bind _topboxpatternscale (Variables|Design_TopBox|GetTopBoxPatternScale))
  (bind _returnvalue (Transformation|GetWorldLocation _scene))
  (Utilities|FlowControl|Sequence
    (:then_0
      (if (Variables|Default|GetLockY)
        ;[1 0 0] Lock Y at 0
        (Transformation|SetWorldLocation (Variables|Default|GetScene) (Math|Vector|MakeVector (.x _returnvalue) 0.0 (.z _returnvalue)) false false)))
    (:then_1
      ;[0 1 0] Breakable Box Material Setup
      (bind _returnvalue_2 (Rendering|Material|CreateDynamicMaterialInstance (Variables|Default|GetBreakableBox) 1 "/Game/PlatformTools/LevelObjects/GameObjects/Boxes/Materials/MI_BoxEdge.MI_BoxEdge" "None" :!class /Script/Engine.PrimitiveComponent))
      (Variables|Design_Breakable|SetBreakableBoxEdgeMI _returnvalue_2)
      (bind _returnvalue_3 (Rendering|Material|CreateDynamicMaterialInstance (Variables|Default|GetBreakableBox) 0 "/Game/PlatformTools/LevelObjects/GameObjects/Boxes/Materials/MI_BoxPattern.MI_BoxPattern" "None" :!class /Script/Engine.PrimitiveComponent))
      (Variables|Design_Breakable|SetBreakableBoxPatternMI _returnvalue_3)
      (Rendering|Material|SetVectorParameterValue (Variables|Design_Breakable|GetBreakableBoxEdgeMI) "BaseColor" (Variables|Design_Breakable|GetBreakableEdgeColor) :!class /Script/Engine.MaterialInstanceDynamic)
      (Rendering|Material|SetVectorParameterValue (Variables|Design_Breakable|GetBreakableBoxPatternMI) "BaseColor" (Variables|Design_Breakable|GetBreakablePatternColor) :!class /Script/Engine.MaterialInstanceDynamic)
      (Rendering|Material|SetTextureParameterValue (Variables|Design_Breakable|GetBreakableBoxPatternMI) "PatternTexture" (Variables|Design_Breakable|GetBreakablePatternTexture))
      (Rendering|Material|SetVectorParameterValue (Variables|Design_Breakable|GetBreakableBoxPatternMI) "PatternOffset" (Utilities|Struct|MakeLinearColor (.x _breakablepatternoffset) (.y _breakablepatternoffset) 0.0 0.0) :!class /Script/Engine.MaterialInstanceDynamic)
      (Rendering|Material|SetVectorParameterValue (Variables|Design_Breakable|GetBreakableBoxPatternMI) "PatternScale" (Utilities|Struct|MakeLinearColor (.x _breakablepatternscale) (.y _breakablepatternscale) 0.0 0.0) :!class /Script/Engine.MaterialInstanceDynamic))
    (:then_2
      ;[0 1 0] Top Box Material Setup
      (bind _returnvalue_4 (Rendering|Material|CreateDynamicMaterialInstance (Variables|Default|GetTopBox) 1 "/Game/PlatformTools/LevelObjects/GameObjects/Boxes/Materials/MI_BoxEdge.MI_BoxEdge" "None" :!class /Script/Engine.PrimitiveComponent))
      (Variables|Design_TopBox|SetTopBoxEdgeMI _returnvalue_4)
      (bind _returnvalue_5 (Rendering|Material|CreateDynamicMaterialInstance (Variables|Default|GetTopBox) 0 "/Game/PlatformTools/LevelObjects/GameObjects/Boxes/Materials/MI_BoxPattern.MI_BoxPattern" "None" :!class /Script/Engine.PrimitiveComponent))
      (Variables|Design_TopBox|SetTopBoxPatternMI _returnvalue_5)
      (Rendering|Material|SetVectorParameterValue (Variables|Design_TopBox|GetTopBoxEdgeMI) "BaseColor" (Variables|Design_TopBox|GetTopBoxEdgeColor) :!class /Script/Engine.MaterialInstanceDynamic)
      (Rendering|Material|SetVectorParameterValue (Variables|Design_TopBox|GetTopBoxPatternMI) "BaseColor" (Variables|Design_TopBox|GetTopBoxPatternColor) :!class /Script/Engine.MaterialInstanceDynamic)
      (Rendering|Material|SetTextureParameterValue (Variables|Design_TopBox|GetTopBoxPatternMI) "PatternTexture" (Variables|Design_TopBox|GetTopBoxPatternTexture))
      (Rendering|Material|SetVectorParameterValue (Variables|Design_TopBox|GetTopBoxPatternMI) "PatternOffset" (Utilities|Struct|MakeLinearColor (.x _topboxpatternoffset) (.y _topboxpatternoffset) 0.0 0.0) :!class /Script/Engine.MaterialInstanceDynamic)
      (Rendering|Material|SetVectorParameterValue (Variables|Design_TopBox|GetTopBoxPatternMI) "PatternScale" (Utilities|Struct|MakeLinearColor (.x _topboxpatternscale) (.y _topboxpatternscale) 0.0 0.0) :!class /Script/Engine.MaterialInstanceDynamic))
    (:then_3
      ;[0 1 0] Top Box Material Setup
      (bind _returnvalue_6 (Rendering|Material|CreateDynamicMaterialInstance (Variables|Default|GetBottomBox) 1 "/Game/PlatformTools/LevelObjects/GameObjects/Boxes/Materials/MI_BoxEdge.MI_BoxEdge" "None" :!class /Script/Engine.PrimitiveComponent))
      (Variables|Design_BottomBox|SetBottomBoxEdgeMI _returnvalue_6)
      (bind _returnvalue_7 (Rendering|Material|CreateDynamicMaterialInstance (Variables|Default|GetBottomBox) 0 "/Game/PlatformTools/LevelObjects/GameObjects/Boxes/Materials/MI_BoxPattern.MI_BoxPattern" "None" :!class /Script/Engine.PrimitiveComponent))
      (Variables|Design_BottomBox|SetBottomBoxPatternMI _returnvalue_7)
      (Rendering|Material|SetVectorParameterValue (Variables|Design_BottomBox|GetBottomBoxEdgeMI) "BaseColor" (Variables|Design_BottomBox|GetBottomBoxEdgeColor) :!class /Script/Engine.MaterialInstanceDynamic)
      (Rendering|Material|SetVectorParameterValue (Variables|Design_BottomBox|GetBottomBoxPatternMI) "BaseColor" (Variables|Design_BottomBox|GetBottomBoxPatternColor) :!class /Script/Engine.MaterialInstanceDynamic)
      (Rendering|Material|SetTextureParameterValue (Variables|Design_BottomBox|GetBottomBoxPatternMI) "PatternTexture" (Variables|Design_BottomBox|GetBottomBoxPatternTexture))
      (Rendering|Material|SetVectorParameterValue (Variables|Design_BottomBox|GetBottomBoxPatternMI) "PatternOffset" (Utilities|Struct|MakeLinearColor (.x _bottomboxpatternoffset) (.y _bottomboxpatternoffset) 0.0 0.0) :!class /Script/Engine.MaterialInstanceDynamic)
      (Rendering|Material|SetVectorParameterValue (Variables|Design_BottomBox|GetBottomBoxPatternMI) "PatternScale" (Utilities|Struct|MakeLinearColor (.x _bottomboxpatternscale) (.y _bottomboxpatternscale) 0.0 0.0) :!class /Script/Engine.MaterialInstanceDynamic))))