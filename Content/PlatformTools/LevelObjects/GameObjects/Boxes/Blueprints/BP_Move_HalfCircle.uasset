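; Platform level object that swings a configurable mesh back and forth along an arc around a pivot, per its name a half circle.
; A timeline, rate-scaled by JourneyTime, drives pivot pitch from StartAngle and reverses on each finish, optionally keeping the mesh unrotated.
; The construction script sets arm length, scales the Circle to match, optionally locks Y to zero, and builds dynamic materials with color and pattern overrides.
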(event Custom|Rotate
  ;[0 1 0] Plays Timeline and Handles Mesh Position
  (if (Variables|Default|GetForward)
    (bind _angle (Timeline|RotationTimeline PlayFromStart)
      (:Update
        (Transformation|SetWorldRotation (Variables|Default|GetPivot) (Math|Rotator|MakeRotator 0.0 (+ _angle (Variables|Default|GetStartAngle)) 0.0) false false)
        (if (Variables|Default|GetLockRotation%28Y/Pitch%29)
          (Transformation|SetWorldRotation (Variables|Default|GetStaticMesh) "0, 0, 0" false false)))
      (:Finished
        (Variables|Default|SetForward (not (Variables|Default|GetForward)))
        (CallFunction|Rotate)))
    (else
      (Timeline|RotationTimeline ReverseFromEnd))))

(event EventBeginPlay
  ;[0 1 0] Setup Timeline
  (Components|Timeline|SetPlayRate (Variables|Default|GetRotationTimeline) (/ 1.0 (Variables|Default|GetJourneyTime)))
  (CallFunction|Rotate))

(fn ConstructionScript
  (bind _length (Variables|Default|GetLength))
  (bind _scene (Variables|Default|GetScene))
  (bind _returnvalue (Transformation|GetWorldLocation _scene))
  (bind _returnvalue_2 (/ _length 1e+02))
  (Utilities|FlowControl|Sequence
    (:then_0
      (if (Variables|Default|GetLockY)
        ;[1 0 0] Lock Y at 0
        (Transformation|SetWorldLocation (Variables|Default|GetScene) (Math|Vector|MakeVector (.x _returnvalue) 0.0 (.z _returnvalue)) false false)))
    (:then_1
      ;[0 1 0] Set up Rotation, Location and Material Instances
      (Transformation|SetWorldRotation (Variables|Default|GetPivot) (Math|Rotator|MakeRotator 0.0 (Variables|Default|GetStartAngle) 0.0) false false)
      (Transformation|SetRelativeLocation (Variables|Default|GetStaticMesh) (Math|Vector|MakeVector (Variables|Default|GetLength) 0.0 0.0) false false)
      (Transformation|SetRelativeScale3D (Variables|Default|GetCircle) (Math|Vector|MakeVector _returnvalue_2 _returnvalue_2 1.0))
      (Components|StaticMesh|SetStaticMesh (Variables|Default|GetStaticMesh) (Variables|Design|GetMesh))
      (for (_array_element _array_index) (Variables|Design|GetMaterialInstances)
        (bind _returnvalue_3 (Rendering|Material|CreateDynamicMaterialInstance (Variables|Default|GetStaticMesh) _array_index _array_element "None" :!class /Script/Engine.PrimitiveComponent))
        (Rendering|Material|SetVectorParameterValue _returnvalue_3 "BaseColor" (Utilities|Array|Get(acopy) (Variables|Design|GetMIColorOverrides) _array_index) :!class /Script/Engine.MaterialInstanceDynamic)
        (if (== _array_index (Variables|Design|GetPatternTextureElement))
          (Rendering|Material|SetTextureParameterValue _returnvalue_3 "PatternTexture" (Variables|Design|GetPatternTexture))))
      (if (Variables|Default|GetLockRotation%28Y/Pitch%29)
        (Transformation|SetWorldRotation (Variables|Default|GetStaticMesh) "0, 0, 0" false false)))))