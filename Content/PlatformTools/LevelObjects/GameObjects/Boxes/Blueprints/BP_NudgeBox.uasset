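; Platformer box that releases a configurable prize the first time the player overlaps it.
; On trigger it plays a sound, recolors, spawns the prize and runs a timeline that nudges the box and moves the prize along a spline.
; The construction script locks Y, line-traces height above ground, optionally matches colors to the prize class, and builds dynamic materials, an editor billboard and the spline.
; Double Jump and Shield prizes can be made perpetual.
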(event OnComponentBeginOverlap(Box)
  (params (OverlappedComponent :type Primitive%20Component%20Object%20Reference) (OtherActor :type Actor%20Object%20Reference) (OtherComp :type Primitive%20Component%20Object%20Reference) (OtherBodyIndex :type Integer) (bFromSweep :type Boolean) (SweepResult :type Hit%20Result%20Structure%20%28by%20ref%29))
  ;[0 1 0] Setup Prize and Animations When Box is Nudged
  (if (== OtherActor (Game|GetPlayerCharacter 0))
    (Utilities|FlowControl|DoOnce false
      (:Completed
        (Audio|PlaySound2D (Variables|Default|GetSoundWave) 1.0 1.0 0.0 0 0)
        (Rendering|Material|SetVectorParameterValue (Variables|Default|GetBoxEdgeMatInst) "BaseColor" (Variables|Design|GetNudgedEdgeColor) :!class /Script/Engine.MaterialInstanceDynamic)
        (Rendering|Material|SetVectorParameterValue (Variables|Default|GetBoxPatternMatInst) "BaseColor" (Variables|Design|GetNudgedPatternColor) :!class /Script/Engine.MaterialInstanceDynamic)
        (bind _returnvalue (Game|SpawnActorfromClass (Variables|Default|GetPrizeClass) (Math|Transform|MakeTransform (Transformation|GetWorldLocation (Variables|Default|GetScene)) "0, 0, 0" "1,1,1") "Undefined" 0 0))
        (Variables|Default|SetActorRef _returnvalue)
        (CallFunction|SetPerpetual)
        (Components|Timeline|SetPlayRate (Variables|Default|GetTimeline) (/ 1.0 (Variables|Default|GetPlayTime%20%28Secs%29)))
        (bind (_direction _prizeloc _nudgeboxloc) (Timeline|Timeline PlayFromStart)
          (:Update
            (Utilities|IsValid _returnvalue
              (:Is%20Valid
                (Transformation|SetActorLocation _returnvalue (Math|Vector|MakeVector (.x (Spline|GetLocationatDistanceAlongSpline (Variables|Default|GetSpline) (* _prizeloc (Spline|GetSplineLength (Variables|Default|GetSpline))) "World")) 0.0 (.z (Spline|GetLocationatDistanceAlongSpline (Variables|Default|GetSpline) (* _prizeloc (Spline|GetSplineLength (Variables|Default|GetSpline))) "World"))) false false)
                (Transformation|SetRelativeLocation (Variables|Default|GetStaticMesh) (Math|Vector|Lerp(Vector) "0, 0, 0" (Variables|Default|GetNudgeBoxOffset) _nudgeboxloc) false false)))))))))

(event EventBeginPlay
  ;[0 1 0] Turn Off Billboard When Game Starts
  (Rendering|SetVisibility (Variables|Default|GetMaterialBillboard) false false))

(fn ConstructionScript
  (Utilities|FlowControl|Sequence
    (:then_0
      ;[0 1 0] Setup Locks for Y and Z
      (CallFunction|LockYandZ))
    (:then_1
      (if (Variables|Default|GetSmartColors)
        ;[0 1 0] Apply Smart Colors if there is a match in the SmartDefinitions table
        (for (_array_element _array_index) (Variables|Default|GetSmartDefinitions)
          (if (== (.PrizeClass (Utilities|Struct|BreakStruct_SmartColors _array_element)) (Variables|Default|GetPrizeClass))
            (Variables|Design|SetPatternColor (.PatternColor (Utilities|Struct|BreakStruct_SmartColors (Utilities|Array|Get(acopy) (Variables|Default|GetSmartDefinitions) _array_index))))
            (Variables|Design|SetEdgeColor (.EdgeColor (Utilities|Struct|BreakStruct_SmartColors (Utilities|Array|Get(acopy) (Variables|Default|GetSmartDefinitions) _array_index))))
            (Variables|Design|SetNudgedEdgeColor (.NudgedEdgeColor (Utilities|Struct|BreakStruct_SmartColors (Utilities|Array|Get(acopy) (Variables|Default|GetSmartDefinitions) _array_index))))
            (Variables|Design|SetNudgedPatternColor (.NudgedPatternColor (Utilities|Struct|BreakStruct_SmartColors (Utilities|Array|Get(acopy) (Variables|Default|GetSmartDefinitions) _array_index))))
            (Variables|Design|SetPatternTexture (.PatternTexture (Utilities|Struct|BreakStruct_SmartColors (Utilities|Array|Get(acopy) (Variables|Default|GetSmartDefinitions) _array_index))))
            (Variables|Design|SetPatternOffset (.PatternOffset (Utilities|Struct|BreakStruct_SmartColors (Utilities|Array|Get(acopy) (Variables|Default|GetSmartDefinitions) _array_index))))
            (Variables|Design|SetPatternScale (.PatternScale (Utilities|Struct|BreakStruct_SmartColors (Utilities|Array|Get(acopy) (Variables|Default|GetSmartDefinitions) _array_index))))))))
    (:then_2
      ;[0 0 1] Setup Dynamic Materials and Textures
      (bind _returnvalue (Rendering|Material|CreateDynamicMaterialInstance (Variables|Default|GetStaticMesh) 1 "/Game/PlatformTools/LevelObjects/GameObjects/Boxes/Materials/MI_BoxEdge.MI_BoxEdge" "None" :!class /Script/Engine.PrimitiveComponent))
      (Variables|Default|SetBoxEdgeMatInst _returnvalue)
      (bind _returnvalue_2 (Rendering|Material|CreateDynamicMaterialInstance (Variables|Default|GetStaticMesh) 0 "/Game/PlatformTools/LevelObjects/GameObjects/Boxes/Materials/MI_BoxPattern.MI_BoxPattern" "None" :!class /Script/Engine.PrimitiveComponent))
      (Variables|Default|SetBoxPatternMatInst _returnvalue_2)
      (Rendering|Material|SetVectorParameterValue (Variables|Default|GetBoxEdgeMatInst) "BaseColor" (Variables|Design|GetEdgeColor) :!class /Script/Engine.MaterialInstanceDynamic)
      (Rendering|Material|SetVectorParameterValue (Variables|Default|GetBoxPatternMatInst) "BaseColor" (Variables|Design|GetPatternColor) :!class /Script/Engine.MaterialInstanceDynamic)
      (Rendering|Material|SetTextureParameterValue (Variables|Default|GetBoxPatternMatInst) "PatternTexture" (Variables|Design|GetPatternTexture))
      (Rendering|Material|SetVectorParameterValue (Variables|Default|GetBoxPatternMatInst) "PatternOffset" (Utilities|Struct|MakeLinearColor (.x (Variables|Design|GetPatternOffset)) (.y (Variables|Design|GetPatternOffset)) 0.0 0.0) :!class /Script/Engine.MaterialInstanceDynamic)
      (Rendering|Material|SetVectorParameterValue (Variables|Default|GetBoxPatternMatInst) "PatternScale" (Utilities|Struct|MakeLinearColor (.x (Variables|Design|GetPatternScale)) (.y (Variables|Design|GetPatternScale)) 0.0 0.0) :!class /Script/Engine.MaterialInstanceDynamic)
      (Transformation|SetRelativeLocation (Variables|Default|GetMaterialBillboard) (Variables|Default|GetPrizeOffset) false false)
      (bind _returnvalue_3 (Rendering|Material|CreateDynamicMaterialInstance (Variables|Default|GetMaterialBillboard) 0 "/Game/PlatformTools/LevelObjects/GameObjects/Boxes/Materials/MI_Billboard.MI_Billboard" "None" :!class /Script/Engine.PrimitiveComponent))
      (Rendering|Material|SetVectorParameterValue _returnvalue_3 "Color" (Variables|Design|GetEdgeColor) :!class /Script/Engine.MaterialInstanceDynamic))
    (:then_3
      ;[1 1 0] Setup Spline Points for the Prize path
      (Spline|SetSplinePoints (Variables|Default|GetSpline) (Utilities|Array|MakeArray "0, 0, 0" (Math|Vector|MakeVector (/ (.x (Variables|Default|GetPrizeOffset)) 2.0) 0.0 1e+02) (Variables|Default|GetPrizeOffset)) "Local" true))))

(fn SetPerpetual
  ;[0 1 0] Setup Perpetual Power Up If Checked
  (if (Variables|Default|GetPerpetualPowerUp)
    (switch string (Utilities|GetClassDisplayName (Variables|Default|GetPrizeClass))
      (:BP_DoubleJump_C
        (bind _asbp_double_jump (Utilities|Casting|CastToBP_DoubleJump (Variables|Default|GetActorRef)))
        (Utilities|IsValid _asbp_double_jump
          (:Is%20Valid
            (Variables|/Game/PlatformTools/LevelObjects/GameObjects/Collectables/Blueprints/BP_DoubleJump.BP_DoubleJump_C|SetPerpetual _asbp_double_jump true))))
      (:BP_Shield_C
        (bind _asbp_shield (Utilities|Casting|CastToBP_Shield (Variables|Default|GetActorRef)))
        (Utilities|IsValid _asbp_shield
          (:Is%20Valid
            (Variables|/Game/PlatformTools/LevelObjects/GameObjects/Collectables/Blueprints/BP_Shield.BP_Shield_C|SetPerpetual _asbp_shield true)))))))

(fn LockYandZ
  (bind _scene (Variables|Default|GetScene))
  (bind _returnvalue (Transformation|GetWorldLocation _scene))
  (bind (_x _y _z) (Math|Vector|BreakVector _returnvalue))
  ;[0 1 0] Use Line Trace to Fix Height from Ground
  (bind _outhit (Collision|LineTraceForObjects _returnvalue (+ _returnvalue "0, 0,-2000.000000") (Utilities|Array|MakeArray "ObjectTypeQuery1") false 0 "None"))
  (if (Variables|Default|GetLockY)
    (Variables|Default|SetYTemp 0.0)
    (else
      (Variables|Default|SetYTemp _y)))
  (if (Variables|Default|GetLockZ)
    (Transformation|SetWorldLocation (Variables|Default|GetScene) (+ (Math|Vector|MakeVector _x (Variables|Default|GetYTemp) (.z (.impactpoint _outhit))) (Math|Vector|MakeVector 0.0 0.0 (Variables|Default|GetZHeight))) false false)
    (else
      (Transformation|SetWorldLocation (Variables|Default|GetScene) (Math|Vector|MakeVector _x (Variables|Default|GetYTemp) _z) false false))))