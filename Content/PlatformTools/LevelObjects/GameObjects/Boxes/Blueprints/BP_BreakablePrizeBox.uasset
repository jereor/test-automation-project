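; Breakable prize box that, on first player overlap, runs a color change, then bursts into a physics-enabled BP_SplitBox with a sound and reveals its prize.
; Construction snaps it to a locked Y and traced ground height, builds dynamic materials, and spawns the hidden prize as a child actor.
; Optional SmartColors styles the box from a table keyed by prize class.
; BeginPlay can flag Double Jump or Shield prizes as perpetual.
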(event OnComponentBeginOverlap(Box)
  (params (OverlappedComponent :type Primitive%20Component%20Object%20Reference) (OtherActor :type Actor%20Object%20Reference) (OtherComp :type Primitive%20Component%20Object%20Reference) (OtherBodyIndex :type Integer) (bFromSweep :type Boolean) (SweepResult :type Hit%20Result%20Structure%20%28by%20ref%29))
  ;[0 1 0] Start Color Change on Timeline when the Player Overlaps, Explode the Box and Play the Sound
  (if (== OtherActor (Game|GetPlayerCharacter 0))
    (Utilities|FlowControl|DoOnce false
      (:Completed
        (Components|Timeline|SetPlayRate (Variables|Default|GetChangeColor) (/ (Components|Timeline|GetTimelineLength (Variables|Default|GetChangeColor)) (Variables|Default|GetPlayback%20Time)))
        (bind _time (Timeline|ChangeColor PlayFromStart)
          (:Update
            (Rendering|Material|SetVectorParameterValue (Variables|Design|GetBreakableBoxEdgeMI) "BaseColor" (Math|Curves|GetLinearColorValue (Variables|Default|GetCurveLinearColor) _time) :!class /Script/Engine.MaterialInstanceDynamic)
            (Rendering|Material|SetVectorParameterValue (Variables|Design|GetBreakableBoxPatternMI) "BaseColor" (Math|Curves|GetLinearColorValue (Variables|Default|GetCurveLinearColor) _time) :!class /Script/Engine.MaterialInstanceDynamic))
          (:Finished
            (Components|DestroyComponent (Variables|Default|GetBreakableBox))
            (Rendering|SetVisibility (Variables|Default|GetSplitBox) true true)
            (bind _asbp_split_box (Utilities|Casting|CastToBP_SplitBox (Variables|/Script/Engine.ChildActorComponent|GetChildActor (Variables|Default|GetSplitBox))))
            (Default|EnablePhysics _asbp_split_box)
            (Audio|PlaySound2D (Variables|Default|GetSoundWave) 1.0 1.0 0.0 0 0)))))))

(event EventBeginPlay
  ;[0 1 0] Setup Perpetual Power Ups
  (CallFunction|SetPerpetual))

(fn ConstructionScript
  (Utilities|FlowControl|Sequence
    (:then_0
      ;[1 0 0] Set Y, Z based on LockY, LockZ and ZHeight
      (CallFunction|LockYandZ))
    (:then_1
      (if (Variables|Default|GetSmartColors)
        ;[0 1 0] Apply Smart Colors if there is a match in the SmartDefinitions table
        (for (_array_element _array_index) (Variables|Default|GetSmartDefinitions)
          (if (== (.PrizeClass (Utilities|Struct|BreakStruct_SmartColors _array_element)) (Variables|Default|GetPrizeClass))
            (Variables|Design|SetBreakablePatternColor (.PatternColor (Utilities|Struct|BreakStruct_SmartColors (Utilities|Array|Get(acopy) (Variables|Default|GetSmartDefinitions) _array_index))))
            (Variables|Design|SetBreakableEdgeColor (.EdgeColor (Utilities|Struct|BreakStruct_SmartColors (Utilities|Array|Get(acopy) (Variables|Default|GetSmartDefinitions) _array_index))))
            (Variables|Design|SetBreakablePatternTexture (.PatternTexture (Utilities|Struct|BreakStruct_SmartColors (Utilities|Array|Get(acopy) (Variables|Default|GetSmartDefinitions) _array_index))))
            (Variables|Design|SetBreakablePatternOffset (.PatternOffset (Utilities|Struct|BreakStruct_SmartColors (Utilities|Array|Get(acopy) (Variables|Default|GetSmartDefinitions) _array_index))))
            (Variables|Design|SetBreakablePatternScale (.PatternScale (Utilities|Struct|BreakStruct_SmartColors (Utilities|Array|Get(acopy) (Variables|Default|GetSmartDefinitions) _array_index))))))))
    (:then_2
      ;[0 1 0] Breakable Box Material Setup
      (bind _returnvalue (Rendering|Material|CreateDynamicMaterialInstance (Variables|Default|GetBreakableBox) 1 "/Game/PlatformTools/LevelObjects/GameObjects/Boxes/Materials/MI_BoxEdge.MI_BoxEdge" "None" :!class /Script/Engine.PrimitiveComponent))
      (Variables|Design|SetBreakableBoxEdgeMI _returnvalue)
      (bind _returnvalue_2 (Rendering|Material|CreateDynamicMaterialInstance (Variables|Default|GetBreakableBox) 0 "/Game/PlatformTools/LevelObjects/GameObjects/Boxes/Materials/MI_BoxPattern.MI_BoxPattern" "None" :!class /Script/Engine.PrimitiveComponent))
      (Variables|Design|SetBreakableBoxPatternMI _returnvalue_2)
      (Rendering|Material|SetVectorParameterValue (Variables|Design|GetBreakableBoxEdgeMI) "BaseColor" (Variables|Design|GetBreakableEdgeColor) :!class /Script/Engine.MaterialInstanceDynamic)
      (Rendering|Material|SetVectorParameterValue (Variables|Design|GetBreakableBoxPatternMI) "BaseColor" (Variables|Design|GetBreakablePatternColor) :!class /Script/Engine.MaterialInstanceDynamic)
      (Rendering|Material|SetTextureParameterValue (Variables|Design|GetBreakableBoxPatternMI) "PatternTexture" (Variables|Design|GetBreakablePatternTexture))
      (Rendering|Material|SetVectorParameterValue (Variables|Design|GetBreakableBoxPatternMI) "PatternOffset" (Utilities|Struct|MakeLinearColor (.x (Variables|Design|GetBreakablePatternOffset)) (.y (Variables|Design|GetBreakablePatternOffset)) 0.0 0.0) :!class /Script/Engine.MaterialInstanceDynamic)
      (Rendering|Material|SetVectorParameterValue (Variables|Design|GetBreakableBoxPatternMI) "PatternScale" (Utilities|Struct|MakeLinearColor (.x (Variables|Design|GetBreakablePatternScale)) (.y (Variables|Design|GetBreakablePatternScale)) 0.0 0.0) :!class /Script/Engine.MaterialInstanceDynamic))
    (:then_3
      ;[1 1 0] Setup the Prize
      (ChildActorComponent|SetChildActorClass (Variables|Default|GetPrize) (Variables|Default|GetPrizeClass))
      (Rendering|SetVisibility (Variables|Default|GetPrize) false true))))

(fn SetPerpetual
  ;[0 1 0] Decides Whether a Perpetual Power Up Is Required (Double Jump or Shield) and Applies it to the Child Actor
  (if (Variables|Default|GetPerpetualPowerUp)
    (switch string (Utilities|GetClassDisplayName (Variables|Default|GetPrizeClass))
      (:BP_DoubleJump_C
        (bind _asbp_double_jump (Utilities|Casting|CastToBP_DoubleJump (Variables|/Script/Engine.ChildActorComponent|GetChildActor (Variables|Default|GetPrize))))
        (Utilities|IsValid _asbp_double_jump
          (:Is%20Valid
            (Variables|/Game/PlatformTools/LevelObjects/GameObjects/Collectables/Blueprints/BP_DoubleJump.BP_DoubleJump_C|SetPerpetual _asbp_double_jump true))))
      (:BP_Shield_C
        (bind _asbp_shield (Utilities|Casting|CastToBP_Shield (Variables|/Script/Engine.ChildActorComponent|GetChildActor (Variables|Default|GetPrize))))
        (Utilities|IsValid _asbp_shield
          (:Is%20Valid
            (Variables|/Game/PlatformTools/LevelObjects/GameObjects/Collectables/Blueprints/BP_Shield.BP_Shield_C|SetPerpetual _asbp_shield true)))))))

(fn LockYandZ
  (bind _scene (Variables|Default|GetScene))
  (bind _returnvalue (Transformation|GetWorldLocation _scene))
  (bind (_x _y _z) (Math|Vector|BreakVector _returnvalue))
  ;[0 1 0] Use Line Trace to Fix Height from Ground
  (bind _outhit (Collision|LineTraceForObjects _returnvalue (+ _returnvalue "0, 0,-2000.000000") (Utilities|Array|MakeArray "ObjectTypeQuery1") false 0 "None"))
  (if (Variables|Default|GetLockY)
    (Variables|Default|SetYTemp 0.0)
    (else
      (Variables|Default|SetYTemp _y)))
  (if (Variables|Default|GetLockZ)
    (Transformation|SetWorldLocation (Variables|Default|GetScene) (+ (Math|Vector|MakeVector _x (Variables|Default|GetYTemp) (.z (.impactpoint _outhit))) (Math|Vector|MakeVector 0.0 0.0 (Variables|Default|GetZHeight))) false false)
    (else
      (Transformation|SetWorldLocation (Variables|Default|GetScene) (Math|Vector|MakeVector _x (Variables|Default|GetYTemp) _z) false false))))