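; Level object that moves a configurable static mesh along a spline.
; At BeginPlay, the SplineTrack timeline starts from StartPercentage at a rate derived from JourneyTime, setting mesh location by distance along the spline without sweeping.
; The construction script optionally pins world Y to zero, previews the mesh at its start point and builds dynamic materials with color overrides and a pattern texture.
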(event EventBeginPlay
  ;[0 1 0] Start the Timeline for the Spline Movement
  (Components|Timeline|SetPlayRate (Variables|Default|GetSplineTrack) (/ 0.5 (Variables|Default|GetJourneyTime)))
  (Utilities|FlowControl|Sequence
    (:then_0
      (bind _percentage (Timeline|SplineTrack SetNewTime)
        (:Update
          (Transformation|SetWorldLocation (Variables|Default|GetStaticMesh) (Spline|GetLocationatDistanceAlongSpline (Variables|Default|GetSpline) (* _percentage (Spline|GetSplineLength (Variables|Default|GetSpline))) "World") false false))))
    (:then_1
      (Timeline|SplineTrack Play))))

(fn ConstructionScript
  (bind _scene (Variables|Default|GetScene))
  (bind _returnvalue (Transformation|GetWorldLocation _scene))
  (Utilities|FlowControl|Sequence
    (:then_0
      (if (Variables|Default|GetLockY)
        ;[1 0 0] Lock Y at 0
        (Transformation|SetWorldLocation (Variables|Default|GetScene) (Math|Vector|MakeVector (.x _returnvalue) 0.0 (.z _returnvalue)) false false)))
    (:then_1
      ;[0 1 0] Setup Spline, Mesh and Material Instances
      (Transformation|SetWorldTransform (Variables|Default|GetStaticMesh) (Spline|GetTransformatDistanceAlongSpline (Variables|Default|GetSpline) (* (Variables|Default|GetStartPercentage) (Spline|GetSplineLength (Variables|Default|GetSpline))) "World" false) false false)
      (Components|StaticMesh|SetStaticMesh (Variables|Default|GetStaticMesh) (Variables|Design|GetMesh))
      (for (_array_element _array_index) (Variables|Design|GetMaterialInstances)
        (bind _returnvalue_2 (Rendering|Material|CreateDynamicMaterialInstance (Variables|Default|GetStaticMesh) _array_index _array_element "None" :!class /Script/Engine.PrimitiveComponent))
        (Rendering|Material|SetVectorParameterValue _returnvalue_2 "BaseColor" (Utilities|Array|Get(acopy) (Variables|Design|GetMIColorOverrides) _array_index) :!class /Script/Engine.MaterialInstanceDynamic)
        (if (== _array_index (Variables|Design|GetPatternTextureElement))
          (Rendering|Material|SetTextureParameterValue _returnvalue_2 "PatternTexture" (Variables|Design|GetPatternTexture)))))))