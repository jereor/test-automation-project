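; Platform level box that appears to float on water, using scripted motion with physics turned off.
; After a short delay on BeginPlay, it snaps the mesh just below the first BP_Water actor's Scene height.
; A timeline then adds WaveHeight to its Z each update and drives yaw through a rotator lerp.
; The construction script optionally locks Y to zero and builds edge and pattern dynamic materials, scaling the pattern with the mesh.
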(event EventBeginPlay
  (bind _boxmesh (Variables|Default|GetBoxMesh))
  (bind _boxmesh_2 (Variables|Default|GetBoxMesh))
  (bind _returnvalue (Transformation|GetWorldLocation _boxmesh_2))
  (bind _returnvalue_2 (Transformation|GetWorldRotation _boxmesh_2))
  (bind _returnvalue_3 (Transformation|GetWorldLocation _boxmesh))
  ;[0 1 0] Setup The Water BluePrint and The Timeline for Making the Box Appear to Float
  (bind _outactors (Actor|GetAllActorsOfClass "/Game/PlatformTools/LevelObjects/EnvironmentObjects/Water/Blueprints/BP_Water.BP_Water_C"))
  (Variables|Default|SetWaterRef (Utilities|Array|Get(acopy) _outactors))
  (Utilities|FlowControl|Delay 0.2)
  (Utilities|FlowControl|DoOnce false
    (:Completed
      (Physics|SetSimulatePhysics (Variables|Default|GetBoxMesh) false)
      (Transformation|SetWorldLocation (Variables|Default|GetBoxMesh) (Math|Vector|MakeVector (.x _returnvalue_3) (.y _returnvalue_3) (- (.z (Transformation|GetWorldLocation (Variables|/Game/PlatformTools/LevelObjects/EnvironmentObjects/Water/Blueprints/BP_Water.BP_Water_C|GetScene (Utilities|Array|Get(acopy) _outactors)))) 4e+01)) false false)
      (bind _waveheight (Timeline|Timeline_0 Play)
        (:Update
          (Transformation|SetWorldLocationAndRotation (Variables|Default|GetBoxMesh) (Math|Vector|MakeVector (.x _returnvalue) (.y _returnvalue) (+ _waveheight (.z _returnvalue))) (Math|Rotator|MakeRotator (.roll _returnvalue_2) (.pitch _returnvalue_2) (.yaw (Math|Rotator|Lerp(Rotator) "0,-5.000000, 0" "0.000000,5.000000,0.000000" _waveheight))) false false))))))

(fn ConstructionScript
  (bind _boxmesh (Variables|Default|GetBoxMesh))
  (bind _patternscalemultiplier (Variables|Design|GetPatternScaleMultiplier))
  (bind _patternposition (Variables|Design|GetPatternPosition))
  (bind _rootscene (Variables|Default|GetRootScene))
  (bind _returnvalue (Transformation|GetWorldLocation _rootscene))
  (bind _returnvalue_2 (Transformation|GetWorldScale _boxmesh))
  (Utilities|FlowControl|Sequence
    (:then_0
      (if (Variables|Default|GetLockY)
        ;[1 0 0] Lock Y at 0
        (Transformation|SetWorldLocation (Variables|Default|GetRootScene) (Math|Vector|MakeVector (.x _returnvalue) 0.0 (.z _returnvalue)) false false)))
    (:then_1
      ;[0 1 0] Setup Dynamic Material Instances
      (Variables|Design|SetPatternScale (Math|Vector2D|MakeVector2D (* (.x _patternscalemultiplier) (.x _returnvalue_2)) (* (.y _patternscalemultiplier) (.y _returnvalue_2))))
      (bind _returnvalue_3 (Rendering|Material|CreateDynamicMaterialInstance (Variables|Default|GetBoxMesh) 0 "/Game/PlatformTools/LevelObjects/GameObjects/Boxes/Materials/MI_BoxEdge.MI_BoxEdge" "Edge" :!class /Script/Engine.PrimitiveComponent))
      (bind _output_get (Variables|Default|SetDMI_Edge _returnvalue_3))
      (Rendering|Material|SetVectorParameterValue _output_get "BaseColor" (Math|Conversions|ToLinearColor(Color) (Variables|Design|GetEdgeColor)) :!class /Script/Engine.MaterialInstanceDynamic)
      (bind _returnvalue_4 (Rendering|Material|CreateDynamicMaterialInstance (Variables|Default|GetBoxMesh) 1 "/Game/PlatformTools/LevelObjects/GameObjects/Boxes/Materials/MI_BoxPattern.MI_BoxPattern" "Pattern" :!class /Script/Engine.PrimitiveComponent))
      (bind _output_get_2 (Variables|Default|SetDMI_Pattern _returnvalue_4))
      (Rendering|Material|SetVectorParameterValue _output_get_2 "BaseColor" (Math|Conversions|ToLinearColor(Color) (Variables|Design|GetPatternColor)) :!class /Script/Engine.MaterialInstanceDynamic)
      (Rendering|Material|SetVectorParameterValue _output_get_2 "PatternScale" (Utilities|Struct|MakeLinearColor (.x (Variables|Design|GetPatternScale)) (.y (Variables|Design|GetPatternScale)) 0.0 1.0) :!class /Script/Engine.MaterialInstanceDynamic)
      (Rendering|Material|SetVectorParameterValue _output_get_2 "PatternOffset" (Utilities|Struct|MakeLinearColor (.x _patternposition) (.y _patternposition) 0.0 1.0) :!class /Script/Engine.MaterialInstanceDynamic)
      (Rendering|Material|SetTextureParameterValue _output_get_2 "PatternTexture" (Variables|Design|GetPatternTexture)))))