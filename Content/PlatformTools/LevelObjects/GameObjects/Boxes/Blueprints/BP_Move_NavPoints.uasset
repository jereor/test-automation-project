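; Moving platform-tool object whose static mesh travels endlessly through an editable array of NavPoint transforms, beginning at a chosen start point.
; A timeline scaled by JourneyTime lerps the mesh's relative transform along each leg without sweep, then advances the index and wraps.
; The construction script optionally locks world Y to zero, spawns numbered child-actor markers at each point, places the mesh, and applies color and pattern overrides through dynamic materials.
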(event Custom|TraverseNavPoints
  ;[0 1 0] Custom Event used to Move from Point to Point
  (if (>= (Variables|Default|GetIndex) (Variables|Default|GetArrayLength))
    (Variables|Default|SetNextIndex 0)
    (else
      (Variables|Default|SetNextIndex (+ (Variables|Default|GetIndex) 1))))
  (Components|Timeline|SetPlayRate (Variables|Default|GetTimeline_0) (/ 1.0 (Variables|Default|GetJourneyTime)))
  (bind _percentagecomplete (Timeline|Timeline_0 PlayFromStart)
    (:Update
      (Transformation|SetRelativeTransform (Variables|Default|GetStaticMesh) (Math|Transform|Lerp(Transform) (Utilities|Array|Get(acopy) (Variables|Default|GetNavPoints) (Variables|Default|GetIndex)) (Utilities|Array|Get(acopy) (Variables|Default|GetNavPoints) (Variables|Default|GetNextIndex)) _percentagecomplete) false false))
    (:Finished
      (bind _output_get (Variables|Default|SetIndex (+ (Variables|Default|GetIndex) 1)))
      (if (>= _output_get (Variables|Default|GetArrayLength))
        (Variables|Default|SetIndex 0))
      (CallFunction|TraverseNavPoints))))

(event EventBeginPlay
  ;[0 1 0] Get the Nav Points from the Array and Start to Move Between Them
  (Variables|Default|SetArrayLength (Utilities|Array|Length (Variables|Default|GetNavPoints)))
  (Variables|Default|SetIndex (Variables|Default|GetStartNavPoint))
  (CallFunction|TraverseNavPoints))

(fn ConstructionScript
  (bind _rootscene (Variables|Default|GetRootScene))
  (bind _returnvalue (Transformation|GetWorldLocation _rootscene))
  (Utilities|FlowControl|Sequence
    (:then_0
      (if (Variables|Default|GetLockY)
        ;[1 0 0] Lock Y at 0
        (Transformation|SetWorldLocation (Variables|Default|GetRootScene) (Math|Vector|MakeVector (.x _returnvalue) 0.0 (.z _returnvalue)) false false)))
    (:then_1
      ;[0 1 0] Setup a Child Actor for Each Nav Point and Display it in Editor with it's Number
      (for (_array_element _array_index) (Variables|Default|GetNavPoints)
        (AddComponent|AddChildActorComponent false (Math|Transform|MakeTransform (.location _array_element) "0, 0, 0" "1,1,1"))
        (bind _returnvalue_2 (AddComponent|AddChildActorComponent false (Math|Transform|MakeTransform (+ (.location _array_element) "0, 0,50.000000") "0, 0, 0" "1,1,1")))
        (bind _asbp_text_render (Utilities|Casting|CastToBP_TextRender (Variables|/Script/Engine.ChildActorComponent|GetChildActor _returnvalue_2)))
        (Variables|/Game/PlatformTools/Characters/RobotEnemy/ReferencedBP/BP_TextRender.BP_TextRender_C|SetText _asbp_text_render (Utilities|Text|ToText(Integer) _array_index))
        (Default|Construction _asbp_text_render))
      (Transformation|SetRelativeTransform (Variables|Default|GetStaticMesh) (Utilities|Array|Get(acopy) (Variables|Default|GetNavPoints) (Variables|Default|GetStartNavPoint)) false false))
    (:then_2
      ;[0 1 0] Create Dynamic Material Instances
      (Components|StaticMesh|SetStaticMesh (Variables|Default|GetStaticMesh) (Variables|Design|GetMesh))
      (for (_array_element_2 _array_index_2) (Variables|Design|GetMaterialInstances)
        (bind _returnvalue_3 (Rendering|Material|CreateDynamicMaterialInstance (Variables|Default|GetStaticMesh) _array_index_2 _array_element_2 "None" :!class /Script/Engine.PrimitiveComponent))
        (Rendering|Material|SetVectorParameterValue _returnvalue_3 "BaseColor" (Utilities|Array|Get(acopy) (Variables|Design|GetMIColorOverrides) _array_index_2) :!class /Script/Engine.MaterialInstanceDynamic)
        (if (== _array_index_2 (Variables|Design|GetPatternTextureElement))
          (Rendering|Material|SetTextureParameterValue _returnvalue_3 "PatternTexture" (Variables|Design|GetPatternTexture)))))))