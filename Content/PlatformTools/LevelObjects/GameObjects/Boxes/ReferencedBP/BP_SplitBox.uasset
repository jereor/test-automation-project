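; BP_SplitBox is a box built from eight static mesh pieces that can be switched to physics simulation.
; The construction script creates dynamic instances of the edge and inside materials, assigns them to the two material slots on every piece, and tints them with the EdgeColor and InsideColor variables.
; EnablePhysics turns on physics simulation for all eight pieces at once.
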(fn ConstructionScript
  ;[0 1 0] Setup Colors for SplitBox
  (bind _returnvalue (Rendering|Material|CreateDynamicMaterialInstance "/Game/PlatformTools/LevelObjects/GameObjects/Boxes/Materials/MI_SplitBoxEdge.MI_SplitBoxEdge" "None" :!class /Script/Engine.KismetMaterialLibrary))
  (Variables|Default|SetDMI_EdgeColor _returnvalue)
  (bind _returnvalue_2 (Rendering|Material|CreateDynamicMaterialInstance "/Game/PlatformTools/LevelObjects/GameObjects/Boxes/Materials/MI_SplitBoxInside.MI_SplitBoxInside" "None" :!class /Script/Engine.KismetMaterialLibrary))
  (Variables|Default|SetDMI_InsideColor _returnvalue_2)
  (Rendering|Material|SetMaterial (Variables|Default|GetStaticMesh) 0 (Variables|Default|GetDMI_InsideColor))
  (Rendering|Material|SetMaterial (Variables|Default|GetStaticMesh) 1 (Variables|Default|GetDMI_EdgeColor))
  (Rendering|Material|SetVectorParameterValue (Variables|Default|GetDMI_EdgeColor) "BaseColor" (Variables|Design|GetEdgeColor) :!class /Script/Engine.MaterialInstanceDynamic)
  (Rendering|Material|SetVectorParameterValue (Variables|Default|GetDMI_InsideColor) "BaseColor" (Variables|Design|GetInsideColor) :!class /Script/Engine.MaterialInstanceDynamic))

(fn EnablePhysics
  ;[0 1 0] Enable Physics on Pieces
  (Physics|SetSimulatePhysics (Variables|Default|GetStaticMesh1) true))