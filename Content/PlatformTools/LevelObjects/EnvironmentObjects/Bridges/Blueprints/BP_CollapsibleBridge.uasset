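; Collapsible bridge pallet for platform levels that drops under physics a set delay after the player first steps on it.
; A TopBox overlap runs a timeline, rescaled to that delay, that tints the dynamic material from a color curve before collapse.
; BottomBox either destroys the actor on contact, floats it with a bobbing timeline on water, or halts physics on spline ground.
; Construction creates the material instance and optionally locks Y to zero.
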(event OnComponentBeginOverlap(TopBox)
  (params (OverlappedComponent :type Primitive%20Component%20Object%20Reference) (OtherActor :type Actor%20Object%20Reference) (OtherComp :type Primitive%20Component%20Object%20Reference) (OtherBodyIndex :type Integer) (bFromSweep :type Boolean) (SweepResult :type Hit%20Result%20Structure%20%28by%20ref%29))
  ;[0 1 0] Change Pallet Color based on Linear Color Set in External Color Curve (%CurveLinearColor%)
  (if (== OtherActor (Game|GetPlayerCharacter 0))
    (Utilities|IsValid OtherActor
      (:Is%20Valid
        (Utilities|FlowControl|DoOnce false
          (:Completed
            (Components|Timeline|SetPlayRate (Variables|Default|GetChangeColor) (/ (Components|Timeline|GetTimelineLength (Variables|Default|GetChangeColor)) (Variables|Default|GetDelayBeforeCollapse)))
            (bind _time (Timeline|ChangeColor PlayFromStart)
              (:Update
                (Rendering|Material|SetVectorParameterValue (Variables|Default|GetPalletMI) "BaseColor" (Math|Curves|GetLinearColorValue (Variables|Default|GetCurveLinearColor) _time) :!class /Script/Engine.MaterialInstanceDynamic))
              (:Finished
                (Physics|SetSimulatePhysics (Variables|Default|GetPalletMesh) true)))))))))

(event OnComponentBeginOverlap(BottomBox)
  (params (OverlappedComponent :type Primitive%20Component%20Object%20Reference) (OtherActor :type Actor%20Object%20Reference) (OtherComp :type Primitive%20Component%20Object%20Reference) (OtherBodyIndex :type Integer) (bFromSweep :type Boolean) (SweepResult :type Hit%20Result%20Structure%20%28by%20ref%29))
  (bind _palletmesh (Variables|Default|GetPalletMesh))
  (bind _palletmesh_2 (Variables|Default|GetPalletMesh))
  (bind _returnvalue (Transformation|GetWorldLocation _palletmesh))
  (bind _returnvalue_2 (Transformation|GetWorldRotation _palletmesh))
  (bind _returnvalue_3 (Transformation|GetWorldLocation _palletmesh_2))
  ;[0 1 1] Make the Pallet Move with Water on Contact
  (if (Variables|Default|GetDestroyOnContact)
    (Actor|DestroyActor)
    (else
      (Utilities|FlowControl|Sequence
        (:then_0
          (bind _asbp_water (Utilities|Casting|CastToBP_Water OtherActor))
          (Utilities|IsValid _asbp_water
            (:Is%20Valid
              (Variables|Default|SetWaterRef OtherActor)
              (Utilities|FlowControl|Delay 0.2)
              (Utilities|FlowControl|DoOnce false
                (:Completed
                  (Physics|SetSimulatePhysics (Variables|Default|GetPalletMesh) false)
                  (Transformation|SetWorldLocation (Variables|Default|GetPalletMesh) (Math|Vector|MakeVector (.x _returnvalue_3) (.y _returnvalue_3) (- (.z (Transformation|GetWorldLocation (Variables|/Game/PlatformTools/LevelObjects/EnvironmentObjects/Water/Blueprints/BP_Water.BP_Water_C|GetScene _asbp_water))) 4e+01)) false false)
                  (bind _waveheight (Timeline|Timeline_0 Play)
                    (:Update
                      (Transformation|SetWorldLocationAndRotation (Variables|Default|GetPalletMesh) (Math|Vector|MakeVector (.x _returnvalue) (.y _returnvalue) (+ _waveheight (.z _returnvalue))) (Math|Rotator|MakeRotator (.roll _returnvalue_2) (.pitch _returnvalue_2) (.yaw (Math|Rotator|Lerp(Rotator) "0,-5.000000, 0" "0.000000,5.000000,0.000000" _waveheight))) false false))))))))
        (:then_1
          (bind _asbp_ground_spline (Utilities|Casting|CastToBP_GroundSpline OtherActor))
          (Utilities|IsValid _asbp_ground_spline
            (:Is%20Valid
              (Utilities|FlowControl|Delay 0.5)
              (Physics|SetSimulatePhysics (Variables|Default|GetPalletMesh) false))))))))

(fn ConstructionScript
  (bind _rootscene (Variables|Default|GetRootScene))
  (bind _returnvalue (Transformation|GetWorldLocation _rootscene))
  ;[0 1 0] Create a DMI for the Pallet Mesh so color can be changed
  (bind _returnvalue_2 (Rendering|Material|CreateDynamicMaterialInstance (Variables|Default|GetPalletMesh) 0 "/Game/PlatformTools/LevelObjects/EnvironmentObjects/Bridges/Materials/MI_PalletMat_Dark.MI_PalletMat_Dark" "None" :!class /Script/Engine.PrimitiveComponent))
  (Variables|Default|SetPalletMI _returnvalue_2)
  ;[1 0 0] Lock the Y axis to Zero
  (if (Variables|Default|GetLockY)
    (Transformation|SetWorldLocation (Variables|Default|GetRootScene) (Math|Vector|MakeVector (.x _returnvalue) 0.0 (.z _returnvalue)) false false)))