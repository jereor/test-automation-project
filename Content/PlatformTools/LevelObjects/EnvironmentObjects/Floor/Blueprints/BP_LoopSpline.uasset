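; Loop-the-loop floor piece that automatically carries the player around a spline in either direction.
; Construction script optionally locks Y to zero, builds spline meshes with optional edge caps and spawns evenly spaced coins.
; Direction-checked start and end boxes disable input, then run forward or reverse timelines that move the capsule, spin the mesh and flag SplineLoop on the GameInstance.
; Exiting overlaps restore input and action, re-arming both DoOnce gates.
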(event OnComponentBeginOverlap(StartBox)
  (params (OverlappedComponent :type Primitive%20Component%20Object%20Reference) (OtherActor :type Actor%20Object%20Reference) (OtherComp :type Primitive%20Component%20Object%20Reference) (OtherBodyIndex :type Integer) (bFromSweep :type Boolean) (SweepResult :type Hit%20Result%20Structure%20%28by%20ref%29))
  (bind _returnvalue (Game|GetPlayerCharacter 0))
  (bind _returnvalue_2 (Game|GetPlayerCharacter 0))
  (bind _bpplatformercomponent (Variables|Default|GetBPPlatformerComponent))
  (bind _defaultspline (Variables|Default|GetDefaultSpline))
  (bind _capsulecomponent (Variables|/Script/Engine.Character|GetCapsuleComponent _returnvalue))
  ;[1 0 1] StartBox - Guide the Player through the Spline - Check Player Direction, Disable Inputs, Calculate the Player Start and End, Run a Timeline from Start to Finish to Set Player Direction and Rotation
  (if (== OtherActor _returnvalue_2)
    (if (< (.y (Math|Vector|GetForwardVector (Variables|/Script/Engine.Character|GetMesh _returnvalue_2))) 0.0)
      (Variables|/Game/PlatformTools/GameDefinitions/Components/BP_Platformer_Main.BP_Platformer_Main_C|SetIgnoreInputs _bpplatformercomponent true)
      (Variables|Default|SetStartAction (Variables|/Game/PlatformTools/GameDefinitions/Components/BP_Platformer_Main.BP_Platformer_Main_C|GetAction _bpplatformercomponent))
      (Utilities|FlowControl|DoOnce false
        (:Completed
          (Variables|Default|SetStart (Spline|GetDistanceAlongSplineatSplinePoint _defaultspline 1))
          (Variables|Default|SetEnd (Spline|GetDistanceAlongSplineatSplinePoint _defaultspline (- (Spline|GetNumberOfSplinePoints _defaultspline) 1)))
          (bind _asgame_instance_platformer (Utilities|Casting|CastToGameInstance_Platformer (Game|GetGameInstance)))
          (Variables|/Game/PlatformTools/GameDefinitions/GameInstance_Platformer.GameInstance_Platformer_C|SetSplineLoop _asgame_instance_platformer true)
          (Components|Timeline|SetPlayRate (Variables|Default|GetForward_Timeline) (/ 1.0 (Variables|Options|GetTime)))
          (bind (_direction _splinedistance _rotation) (Timeline|Forward_Timeline PlayFromStart)
            (:Update
              (bind _output_get (Variables|Default|SetCurrentDistance (Math|Float|Lerp (Variables|Default|GetStart) (Variables|Default|GetEnd) _splinedistance)))
              (Transformation|SetWorldLocation _capsulecomponent (+ (Spline|GetLocationatDistanceAlongSpline (Variables|Default|GetDefaultSpline) _output_get "World") (Math|Vector|MakeVector 0.0 0.0 (Variables|/Script/Engine.CapsuleComponent|GetCapsuleHalfHeight _capsulecomponent))) false false)
              (Transformation|SetWorldRotation (Variables|/Script/Engine.Character|GetMesh _returnvalue) (Math|Rotator|MakeRotator (Math|Float|Lerp 3.6e+02 0.0 _rotation) 0.0 -9e+01) false false))
            (:Finished
              (bind _asgame_instance_platformer_2 (Utilities|Casting|CastToGameInstance_Platformer (Game|GetGameInstance)))
              (Variables|/Game/PlatformTools/GameDefinitions/GameInstance_Platformer.GameInstance_Platformer_C|SetSplineLoop _asgame_instance_platformer_2 false))))))))

(event OnComponentBeginOverlap(EndBox)
  (params (OverlappedComponent :type Primitive%20Component%20Object%20Reference) (OtherActor :type Actor%20Object%20Reference) (OtherComp :type Primitive%20Component%20Object%20Reference) (OtherBodyIndex :type Integer) (bFromSweep :type Boolean) (SweepResult :type Hit%20Result%20Structure%20%28by%20ref%29))
  (bind _returnvalue (Game|GetPlayerCharacter 0))
  (bind _returnvalue_2 (Game|GetPlayerCharacter 0))
  (bind _bpplatformercomponent (Variables|Default|GetBPPlatformerComponent))
  (bind _defaultspline (Variables|Default|GetDefaultSpline))
  (bind _capsulecomponent (Variables|/Script/Engine.Character|GetCapsuleComponent _returnvalue_2))
  ;[0 1 1] EndBox - Guide the Player through the Spline - Check Player Direction, Disable Inputs, Calculate the Player Start and End, Run a Timeline from Start to Finish to Set Player Direction and Rotation
  (if (== OtherActor _returnvalue)
    (if (> (.y (Math|Vector|GetForwardVector (Variables|/Script/Engine.Character|GetMesh _returnvalue))) 0.0)
      (Variables|/Game/PlatformTools/GameDefinitions/Components/BP_Platformer_Main.BP_Platformer_Main_C|SetIgnoreInputs _bpplatformercomponent true)
      (Variables|Default|SetStartAction (Variables|/Game/PlatformTools/GameDefinitions/Components/BP_Platformer_Main.BP_Platformer_Main_C|GetAction _bpplatformercomponent))
      (Utilities|FlowControl|DoOnce false
        (:Completed
          (Variables|Default|SetStart (Spline|GetDistanceAlongSplineatSplinePoint _defaultspline 1))
          (Variables|Default|SetEnd (Spline|GetDistanceAlongSplineatSplinePoint _defaultspline (- (Spline|GetNumberOfSplinePoints _defaultspline) 1)))
          (bind _asgame_instance_platformer (Utilities|Casting|CastToGameInstance_Platformer (Game|GetGameInstance)))
          (Variables|/Game/PlatformTools/GameDefinitions/GameInstance_Platformer.GameInstance_Platformer_C|SetSplineLoop _asgame_instance_platformer true)
          (Components|Timeline|SetPlayRate (Variables|Default|GetReverse_Timeline) (/ 1.0 (Variables|Options|GetTime)))
          (bind (_direction _splinedistance _rotation) (Timeline|Reverse_Timeline PlayFromStart)
            (:Update
              (bind _output_get (Variables|Default|SetCurrentDistance (Math|Float|Lerp (Variables|Default|GetEnd) (Variables|Default|GetStart) _splinedistance)))
              (Transformation|SetWorldLocation _capsulecomponent (+ (Spline|GetLocationatDistanceAlongSpline (Variables|Default|GetDefaultSpline) _output_get "World") (Math|Vector|MakeVector 0.0 0.0 (Variables|/Script/Engine.CapsuleComponent|GetCapsuleHalfHeight _capsulecomponent))) false false)
              (Transformation|SetWorldRotation (Variables|/Script/Engine.Character|GetMesh _returnvalue_2) (Math|Rotator|MakeRotator (Math|Float|Lerp 3.6e+02 0.0 _rotation) 0.0 9e+01) false false))
            (:Finished
              (bind _asgame_instance_platformer_2 (Utilities|Casting|CastToGameInstance_Platformer (Game|GetGameInstance)))
              (Variables|/Game/PlatformTools/GameDefinitions/GameInstance_Platformer.GameInstance_Platformer_C|SetSplineLoop _asgame_instance_platformer_2 false))))))))

(event OnComponentEndOverlap(EndBox)
  (params (OverlappedComponent :type Primitive%20Component%20Object%20Reference) (OtherActor :type Actor%20Object%20Reference) (OtherComp :type Primitive%20Component%20Object%20Reference) (OtherBodyIndex :type Integer))
  (bind _returnvalue (Game|GetPlayerCharacter 0))
  (bind _bpplatformercomponent (Variables|Default|GetBPPlatformerComponent))
  ;[0 0 1] EndBox - Ensure Smooth Exit of the Overlap Dependent on Player Direction
  (if (== OtherActor _returnvalue)
    (if (< (.y (Math|Vector|GetForwardVector (Variables|/Script/Engine.Character|GetMesh _returnvalue))) 0.0)
      (Variables|/Game/PlatformTools/GameDefinitions/Components/BP_Platformer_Main.BP_Platformer_Main_C|SetIgnoreInputs _bpplatformercomponent false)
      (Variables|/Game/PlatformTools/GameDefinitions/Components/BP_Platformer_Main.BP_Platformer_Main_C|SetAction _bpplatformercomponent (Variables|Default|GetStartAction))
      (CallFunction|ResetStartBox)
      (CallFunction|ResetEndBox))))

(event OnComponentEndOverlap(StartBox)
  (params (OverlappedComponent :type Primitive%20Component%20Object%20Reference) (OtherActor :type Actor%20Object%20Reference) (OtherComp :type Primitive%20Component%20Object%20Reference) (OtherBodyIndex :type Integer))
  (bind _returnvalue (Game|GetPlayerCharacter 0))
  (bind _bpplatformercomponent (Variables|Default|GetBPPlatformerComponent))
  ;[1 0 0] StartBox - Ensure Smooth Exit of the Overlap Dependent on Player Direction
  (if (== OtherActor _returnvalue)
    (if (> (.y (Math|Vector|GetForwardVector (Variables|/Script/Engine.Character|GetMesh _returnvalue))) 0.0)
      (Variables|/Game/PlatformTools/GameDefinitions/Components/BP_Platformer_Main.BP_Platformer_Main_C|SetIgnoreInputs _bpplatformercomponent false)
      (Variables|/Game/PlatformTools/GameDefinitions/Components/BP_Platformer_Main.BP_Platformer_Main_C|SetAction _bpplatformercomponent (Variables|Default|GetStartAction))
      (CallFunction|ResetStartBox)
      (CallFunction|ResetEndBox))))

(event Custom|ResetStartBox
  (bind _returnvalue (Game|GetPlayerCharacter 0))
  (bind _defaultspline (Variables|Default|GetDefaultSpline))
  (bind _capsulecomponent (Variables|/Script/Engine.Character|GetCapsuleComponent _returnvalue))
  ;[1 0 1] StartBox - Guide the Player through the Spline - Check Player Direction, Disable Inputs, Calculate the Player Start and End, Run a Timeline from Start to Finish to Set Player Direction and Rotation
  (Utilities|FlowControl|DoOnce false) ; enters at Reset
)

(event Custom|ResetEndBox
  (bind _returnvalue (Game|GetPlayerCharacter 0))
  (bind _defaultspline (Variables|Default|GetDefaultSpline))
  (bind _capsulecomponent (Variables|/Script/Engine.Character|GetCapsuleComponent _returnvalue))
  ;[0 1 1] EndBox - Guide the Player through the Spline - Check Player Direction, Disable Inputs, Calculate the Player Start and End, Run a Timeline from Start to Finish to Set Player Direction and Rotation
  (Utilities|FlowControl|DoOnce false) ; enters at Reset
)

(event EventBeginPlay
  (bind _returnvalue (Game|GetPlayerCharacter 0))
  (bind _returnvalue_2 (Actor|GetComponentbyClass _returnvalue "/Game/PlatformTools/GameDefinitions/Components/BP_Platformer_Main.BP_Platformer_Main_C"))
  ;[1 1 0] Connect to Platformer_Main Component in Player
  (Utilities|FlowControl|Delay 0.2)
  (Utilities|IsValid _returnvalue_2
    (:Is%20Valid
      (Variables|Default|SetBPPlatformerComponent _returnvalue_2))))

(fn ConstructionScript
  (bind _defaultspline (Variables|Default|GetDefaultSpline))
  (bind _scene (Variables|Default|GetScene))
  (bind _defaultspline_2 (Variables|Default|GetDefaultSpline))
  (bind _defaultspline_3 (Variables|Default|GetDefaultSpline))
  (bind _coinspacing (Variables|Options|GetCoinSpacing))
  (bind _returnvalue (Transformation|GetWorldLocation _scene))
  (bind _returnvalue_2 (Spline|GetDistanceAlongSplineatSplinePoint _defaultspline_2 1))
  (bind _returnvalue_3 (Spline|GetSplineLength _defaultspline_2))
  (bind _returnvalue_4 (Spline|GetNumberOfSplinePoints _defaultspline))
  (bind _returnvalue_5 (- _returnvalue_3 _returnvalue_2))
  (bind (_remainder _returnvalue_6) (Math|Float|Division(WholeandRemainder) _returnvalue_5 _coinspacing))
  (Utilities|FlowControl|Sequence
    (:then_0
      ;[1 0 0] Lock the Y axis to Zero
      (if (Variables|Default|GetLockY)
        (Transformation|SetWorldLocation (Variables|Default|GetScene) (Math|Vector|MakeVector (.x _returnvalue) 0.0 (.z _returnvalue)) false false)))
    (:then_1
      ;[0 1 0] Setup Ground Meshes
      (for _index (range 1 (- _returnvalue_4 2))
        (Utilities|FlowControl|Sequence
          (:then_0
            (bind _returnvalue_7 (AddComponent|AddSplineMeshComponent true (Math|Transform|MakeTransform "0, 0, 0" "0, 0, 0" (Variables|Meshes|GetMeshScale))))
            (SplineMesh|SetStartandEnd _returnvalue_7 (.Location (Spline|GetLocationandTangentatSplinePoint _defaultspline_3 _index "World")) (.Tangent (Spline|GetLocationandTangentatSplinePoint _defaultspline_3 _index "World")) (.Location (Spline|GetLocationandTangentatSplinePoint _defaultspline_3 (+ _index 1) "World")) (.Tangent (Spline|GetLocationandTangentatSplinePoint _defaultspline_3 (+ _index 1) "World")) true :!class /Script/Engine.SplineMeshComponent)
            (Class|SplineMeshComponent|SetStartRoll _returnvalue_7 (Spline|GetRollatSplinePoint _defaultspline_3 _index "World") true)
            (Class|SplineMeshComponent|SetEndRoll _returnvalue_7 (Spline|GetRollatSplinePoint _defaultspline_3 (+ _index 1) "World") true)
            (SplineMesh|SetSplineUpDir _returnvalue_7 (Math|Vector|RotateVectorAroundAxis (Class|SplineComponent|GetDirectionatSplinePoint _defaultspline_3 _index "World") -9e+01 "0.000000,1.000000,0.000000") true)
            (Collision|SetCollisionEnabled _returnvalue_7 "QueryAndPhysics")
            (Collision|SetCollisionObjectType _returnvalue_7 "ECC_WorldDynamic")
            (if (== _index 1)
              (if (Variables|Options|GetEdges)
                (Components|StaticMesh|SetStaticMesh _returnvalue_7 (Variables|Meshes|GetStaticMeshLeftEdge))
                (else
                  (Components|StaticMesh|SetStaticMesh _returnvalue_7 (Variables|Meshes|GetMainMesh) :!label _label)))
              (elif (== _index (- _returnvalue_4 2))
                (if (Variables|Options|GetEdges)
                  (Components|StaticMesh|SetStaticMesh _returnvalue_7 (Variables|Meshes|GetStaticMeshRightEdge))
                  (else
                    (goto _label)))
                (else
                  (goto _label))))))))
    (:then_2
      ;[1 1 0] Setup Automatic Coins
      (if (Variables|Options|GetAutoCoins)
        (bind _output_get (Variables|Default|SetNumCoins _returnvalue_6))
        (for _index_2 (range 0 _output_get)
          (bind _returnvalue_8 (AddComponent|AddChildActorComponent true (Math|Transform|MakeTransform (Spline|GetLocationatDistanceAlongSpline (Variables|Default|GetDefaultSpline) (+ (* _index_2 (Variables|Options|GetCoinSpacing)) _returnvalue_2 (/ _remainder 2.0)) "World") (Math|Rotator|MakeRotator 0.0 (* _index_2 (/ 3.6e+02 (Math|Conversions|ToFloat(Integer) _output_get))) 0.0) "1,1,1")))
          (ChildActorComponent|SetChildActorClass _returnvalue_8 (Variables|Meshes|GetCoinBP)))))))