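; Spline-based floor piece for platform levels, built in the construction script with optional locking to world Y zero.
; Lays colliding spline meshes from point 1 onward, skipping the first segment, matching tangents and roll, with optional left and right edge meshes.
; Optionally spawns evenly spaced, centered coins and randomly offset flowers as child actors along that span.
; Flower placement is unseeded, so it changes on every construction rerun.
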(fn ConstructionScript
  (bind _defaultspline (Variables|Default|GetDefaultSpline))
  (bind _coinspacing (Variables|Options|GetCoinSpacing))
  (bind _defaultspline_2 (Variables|Default|GetDefaultSpline))
  (bind _scene (Variables|Default|GetScene))
  (bind _defaultspline_3 (Variables|Default|GetDefaultSpline))
  (bind _defaultspline_4 (Variables|Default|GetDefaultSpline))
  (bind _plantspacing (Variables|Options|GetPlantSpacing))
  (bind _returnvalue (Transformation|GetWorldLocation _scene))
  (bind _returnvalue_2 (Spline|GetDistanceAlongSplineatSplinePoint _defaultspline_3 1))
  (bind _returnvalue_3 (Spline|GetSplineLength _defaultspline_3))
  (bind _returnvalue_4 (Spline|GetDistanceAlongSplineatSplinePoint _defaultspline 1))
  (bind _returnvalue_5 (Spline|GetSplineLength _defaultspline))
  (bind _returnvalue_6 (Spline|GetNumberOfSplinePoints _defaultspline_2))
  (bind _returnvalue_7 (- _returnvalue_3 _returnvalue_2))
  (bind _returnvalue_8 (- _returnvalue_5 _returnvalue_4))
  (bind (_remainder _returnvalue_9) (Math|Float|Division(WholeandRemainder) _returnvalue_8 _coinspacing))
  (bind (_remainder_2 _returnvalue_10) (Math|Float|Division(WholeandRemainder) _returnvalue_7 _plantspacing))
  (Utilities|FlowControl|Sequence
    (:then_0
      ;[1 0 0] Lock the Y axis to Zero
      (if (Variables|Default|GetLockY)
        (Transformation|SetWorldLocation (Variables|Default|GetScene) (Math|Vector|MakeVector (.x _returnvalue) 0.0 (.z _returnvalue)) false false)))
    (:then_1
      ;[0 1 0] Setup Main Meshes for GroundSpline
      (for _index (range 1 (- _returnvalue_6 2))
        (Utilities|FlowControl|Sequence
          (:then_0
            (bind _returnvalue_11 (AddComponent|AddSplineMeshComponent true (Math|Transform|MakeTransform "0, 0, 0" "0, 0, 0" (Variables|Meshes|GetMeshScale))))
            (SplineMesh|SetStartandEnd _returnvalue_11 (.Location (Spline|GetLocationandTangentatSplinePoint _defaultspline_4 _index "World")) (.Tangent (Spline|GetLocationandTangentatSplinePoint _defaultspline_4 _index "World")) (.Location (Spline|GetLocationandTangentatSplinePoint _defaultspline_4 (+ _index 1) "World")) (.Tangent (Spline|GetLocationandTangentatSplinePoint _defaultspline_4 (+ _index 1) "World")) true :!class /Script/Engine.SplineMeshComponent)
            (Class|SplineMeshComponent|SetStartRoll _returnvalue_11 (Spline|GetRollatSplinePoint _defaultspline_4 _index "World") true)
            (Class|SplineMeshComponent|SetEndRoll _returnvalue_11 (Spline|GetRollatSplinePoint _defaultspline_4 (+ _index 1) "World") true)
            (Collision|SetCollisionEnabled _returnvalue_11 "QueryAndPhysics")
            (if (== _index 1)
              (if (Variables|Options|GetEdges)
                (Components|StaticMesh|SetStaticMesh _returnvalue_11 (Variables|Meshes|GetStaticMeshLeftEdge))
                (else
                  (Components|StaticMesh|SetStaticMesh _returnvalue_11 (Variables|Meshes|GetMainMesh) :!label _label)))
              (elif (== _index (- _returnvalue_6 2))
                (if (Variables|Options|GetEdges)
                  (Components|StaticMesh|SetStaticMesh _returnvalue_11 (Variables|Meshes|GetStaticMeshRightEdge))
                  (else
                    (goto _label)))
                (else
                  (goto _label))))))))
    (:then_2
      ;[1 1 0] Setup Automatic Coins
      (if (Variables|Options|GetAutoCoins)
        (bind _output_get (Variables|Options|SetNumCoins _returnvalue_9))
        (for _index_2 (range 1 _output_get)
          (bind _returnvalue_12 (AddComponent|AddChildActorComponent true (Math|Transform|MakeTransform (+ (Spline|GetLocationatDistanceAlongSpline (Variables|Default|GetDefaultSpline) (+ (* _index_2 (Variables|Options|GetCoinSpacing)) _returnvalue_4 (/ _remainder 2.0)) "World") (Math|Vector|MakeVector 0.0 0.0 (Variables|Options|GetCoinHeight))) "0, 0, 0" "1,1,1")))
          (ChildActorComponent|SetChildActorClass _returnvalue_12 (Variables|Options|GetCoinBP)))))
    (:then_3
      ;[1 0 1] Setup Automatic Flowers - Note that the Flowers will move EACH TIME the Construction Script is run since they are randomized on the Y axis.
      (if (Variables|Options|GetAutoFlowers)
        (bind _output_get_2 (Variables|Options|SetNumPlants _returnvalue_10))
        (for _index_3 (range 0 _output_get_2)
          (bind _returnvalue_13 (AddComponent|AddChildActorComponent true (Math|Transform|MakeTransform (+ (Spline|GetLocationatDistanceAlongSpline (Variables|Default|GetDefaultSpline) (+ (* _index_3 (Variables|Options|GetPlantSpacing)) (/ _remainder_2 2.0) _returnvalue_2 (Math|Random|RandomFloatinRange -5e+01 5e+01)) "World") (Math|Vector|MakeVector 0.0 (Math|Random|RandomFloatinRange -3e+02 3e+02) 1.3e+02)) (Math|Rotator|MakeRotfromX (Spline|GetTangentatDistanceAlongSpline (Variables|Default|GetDefaultSpline) (+ (* _index_3 (Variables|Options|GetPlantSpacing)) (/ _remainder_2 2.0) _returnvalue_2 (Math|Random|RandomFloatinRange -5e+01 5e+01)) "World")) "1,1,1")))
          (ChildActorComponent|SetChildActorClass _returnvalue_13 "/Game/PlatformTools/LevelObjects/EnvironmentObjects/Plants/Blueprints/BP_Flowers.BP_Flowers_C"))))))