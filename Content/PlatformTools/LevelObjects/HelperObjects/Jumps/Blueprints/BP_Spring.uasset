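; Spring jump pad that launches the player on overlap, using the right or left launch velocity according to facing direction.
; Z velocity is always overridden, XY only when the chosen velocity has an X component.
; A timeline animates the cylinder's position and the spring's Z scale, re-arming the DoOnce trigger when finished.
; The construction script optionally locks the spring to Y=0, previews both predicted launch arcs and applies tinted dynamic materials.
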(event OnComponentBeginOverlap(Sphere)
  (params (OverlappedComponent :type Primitive%20Component%20Object%20Reference) (OtherActor :type Actor%20Object%20Reference) (OtherComp :type Primitive%20Component%20Object%20Reference) (OtherBodyIndex :type Integer) (bFromSweep :type Boolean) (SweepResult :type Hit%20Result%20Structure%20%28by%20ref%29))
  (bind _leftlaunchvelocity (Variables|Default|GetLeftLaunchVelocity))
  (bind _rightlaunchvelocity (Variables|Default|GetRightLaunchVelocity))
  ;[0 1 0] Launch the Player with the Appropriate Launch Velocity
  (if (== OtherActor (Game|GetPlayerCharacter 0))
    (Utilities|FlowControl|DoOnce false
      (:Completed
        (if (< (Math|Float|Sign(Float) (.y (Math|Vector|GetForwardVector (Variables|/Script/Engine.Character|GetMesh (Game|GetPlayerCharacter 0))))) 0.0)
          (if (== (.x (Variables|Default|GetRightLaunchVelocity)) 0.0)
            (Character|LaunchCharacter (Game|GetPlayerCharacter 0) _rightlaunchvelocity false true)
            (bind _time (Timeline|0-Max PlayFromStart)
              (:Update
                (Transformation|SetWorldLocation (Variables|Default|GetCylinder) (+ (Transformation|GetWorldLocation (Variables|Default|GetScene)) (Math|Vector|Lerp(Vector) "0, 0, 0" (Variables|Default|GetFinalLocation) _time)) false false)
                (Transformation|SetRelativeScale3D (Variables|Default|GetSpring) (Math|Vector|MakeVector 1.0 1.0 (Math|Float|Lerp 0.0 1.0 _time))))
              (:Finished
                (CallFunction|ResetTimeline)))
            (else
              (Character|LaunchCharacter (Game|GetPlayerCharacter 0) _rightlaunchvelocity true true)
              (Timeline|0-Max PlayFromStart)))
          (elif (== (.x (Variables|Default|GetLeftLaunchVelocity)) 0.0)
            (Character|LaunchCharacter (Game|GetPlayerCharacter 0) _leftlaunchvelocity false true)
            (Timeline|0-Max PlayFromStart)
            (else
              (Character|LaunchCharacter (Game|GetPlayerCharacter 0) _leftlaunchvelocity true true)
              (Timeline|0-Max PlayFromStart))))))))

(event Custom|ResetTimeline
  (bind _leftlaunchvelocity (Variables|Default|GetLeftLaunchVelocity))
  (bind _rightlaunchvelocity (Variables|Default|GetRightLaunchVelocity))
  ;[0 1 0] Launch the Player with the Appropriate Launch Velocity
  (Utilities|FlowControl|DoOnce false) ; enters at Reset
)

(fn ConstructionScript
  (bind _array (Utilities|Array|MakeArray "ObjectTypeQuery3"))
  (bind _scene (Variables|Default|GetScene))
  (bind _scene_2 (Variables|Default|GetScene))
  (bind _returnvalue (Transformation|GetWorldLocation _scene_2))
  (bind _returnvalue_2 (Transformation|GetWorldLocation _scene))
  (Utilities|FlowControl|Sequence
    (:then_0
      (if (Variables|Default|GetLockY)
        ;[1 0 0] Lock Y at 0
        (Transformation|SetWorldLocation (Variables|Default|GetScene) (Math|Vector|MakeVector (.x _returnvalue) 0.0 (.z _returnvalue)) false false)))
    (:then_1
      ;[0 1 0] Display Projectile Path and Setup Material Instances
      (Class|GameplayStatics|BlueprintPredictProjectilePathbyObjectType _returnvalue_2 (Variables|Default|GetRightLaunchVelocity) true 0.0 _array false 0 "ForOneFrame")
      (Class|GameplayStatics|BlueprintPredictProjectilePathbyObjectType _returnvalue_2 (Variables|Default|GetLeftLaunchVelocity) true 0.0 _array false 0 "ForOneFrame")
      (bind _returnvalue_3 (Rendering|Material|CreateDynamicMaterialInstance (Variables|Default|GetCylinder) 0 "/Game/PlatformTools/LevelObjects/GameObjects/Collectables/Materials/MI_Metal_Red.MI_Metal_Red" "None" :!class /Script/Engine.PrimitiveComponent))
      (bind _output_get (Variables|Default|SetCylinderDMI _returnvalue_3))
      (Rendering|Material|SetVectorParameterValue _output_get "BaseColor" (Variables|Design|GetCylinderColor) :!class /Script/Engine.MaterialInstanceDynamic)
      (bind _returnvalue_4 (Rendering|Material|CreateDynamicMaterialInstance (Variables|Default|GetSpring) 0 "/Game/PlatformTools/LevelObjects/GameObjects/Collectables/Materials/MI_Metal_Silver.MI_Metal_Silver" "None" :!class /Script/Engine.PrimitiveComponent))
      (bind _output_get_2 (Variables|Default|SetSpringDMI _returnvalue_4))
      (Rendering|Material|SetVectorParameterValue _output_get_2 "BaseColor" (Variables|Design|GetSpringColor) :!class /Script/Engine.MaterialInstanceDynamic))))