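; BP_PrecisionJump is a trigger volume that overrides the player's jump with authored left and right launch velocities.
; On player overlap, it passes both velocities and a jump location, raised by capsule half-height, to the player's BP_Platformer_Main component and enables precision jump.
; Leaving the box disables it.
; The construction script optionally locks Y to zero and previews both arcs using projectile-path prediction debug drawing.
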(event OnComponentBeginOverlap(Box)
  (params (OverlappedComponent :type Primitive%20Component%20Object%20Reference) (OtherActor :type Actor%20Object%20Reference) (OtherComp :type Primitive%20Component%20Object%20Reference) (OtherBodyIndex :type Integer) (bFromSweep :type Boolean) (SweepResult :type Hit%20Result%20Structure%20%28by%20ref%29))
  (bind _bpplatformercomponent (Variables|Default|GetBPPlatformerComponent))
  ;[0 1 0] Handle Player Jump Overrides
  (if (== OtherActor (Game|GetPlayerCharacter 0))
    (Utilities|IsValid _bpplatformercomponent
      (:Is%20Valid
        (Variables|/Game/PlatformTools/GameDefinitions/Components/BP_Platformer_Main.BP_Platformer_Main_C|SetPrecisionJump _bpplatformercomponent true)
        (Variables|/Game/PlatformTools/GameDefinitions/Components/BP_Platformer_Main.BP_Platformer_Main_C|SetPrecisionJumpVel_Left _bpplatformercomponent (Variables|Default|GetJumpLeftOverride))
        (Variables|/Game/PlatformTools/GameDefinitions/Components/BP_Platformer_Main.BP_Platformer_Main_C|SetPrecisionJumpVel_Right _bpplatformercomponent (Variables|Default|GetJumpRightOverride))
        (Variables|/Game/PlatformTools/GameDefinitions/Components/BP_Platformer_Main.BP_Platformer_Main_C|SetPrecisionJumpLocation _bpplatformercomponent (+ (Transformation|GetWorldLocation (Variables|Default|GetScene)) (Math|Vector|MakeVector 0.0 0.0 (Components|Capsule|GetScaledCapsuleHalfHeight (Variables|/Script/Engine.Character|GetCapsuleComponent (Game|GetPlayerCharacter 0))))))))))

(event OnComponentEndOverlap(Box)
  (params (OverlappedComponent :type Primitive%20Component%20Object%20Reference) (OtherActor :type Actor%20Object%20Reference) (OtherComp :type Primitive%20Component%20Object%20Reference) (OtherBodyIndex :type Integer))
  (bind _bpplatformercomponent (Variables|Default|GetBPPlatformerComponent))
  ;[1 0 0] Disable Precision Jump When Exiting the Collision Area
  (if (== OtherActor (Game|GetPlayerCharacter 0))
    (Utilities|IsValid _bpplatformercomponent
      (:Is%20Valid
        (Variables|/Game/PlatformTools/GameDefinitions/Components/BP_Platformer_Main.BP_Platformer_Main_C|SetPrecisionJump _bpplatformercomponent false)))))

(event EventBeginPlay
  (bind _returnvalue (Game|GetPlayerCharacter 0))
  (bind _returnvalue_2 (Actor|GetComponentbyClass _returnvalue "/Game/PlatformTools/GameDefinitions/Components/BP_Platformer_Main.BP_Platformer_Main_C"))
  ;[1 1 0] Connect to Platformer_Main Component in Player
  (Utilities|FlowControl|Delay 0.2)
  (Utilities|IsValid _returnvalue_2
    (:Is%20Valid
      (Variables|Default|SetBPPlatformerComponent _returnvalue_2))))

(fn ConstructionScript
  (bind _array (Utilities|Array|MakeArray "ObjectTypeQuery3"))
  (bind _scene (Variables|Default|GetScene))
  (bind _scene_2 (Variables|Default|GetScene))
  (bind _returnvalue (Transformation|GetWorldLocation _scene_2))
  (bind _returnvalue_2 (Transformation|GetWorldLocation _scene))
  (Utilities|FlowControl|Sequence
    (:then_0
      (if (Variables|Default|GetLockY)
        ;[1 0 0] Lock Y at 0
        (Transformation|SetWorldLocation (Variables|Default|GetScene) (Math|Vector|MakeVector (.x _returnvalue) 0.0 (.z _returnvalue)) false false)))
    (:then_1
      ;[0 1 0] Show Paths for Left and Right Directions
      (Class|GameplayStatics|BlueprintPredictProjectilePathbyObjectType _returnvalue_2 (Variables|Default|GetJumpRightOverride) true 0.0 _array false 0 "ForOneFrame")
      (Class|GameplayStatics|BlueprintPredictProjectilePathbyObjectType _returnvalue_2 (Variables|Default|GetJumpLeftOverride) true 0.0 _array false 0 "ForOneFrame"))))