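; Checkpoint actor for a platformer that saves the player's respawn transform the first time the player overlaps it.
; The first overlap plays a sound, releases both rope ends, swaps the sphere materials and shows a timed "Check Point" message.
; It writes the spawn transform and zoom setting to the player's BP_Platformer_Main component, cached shortly after BeginPlay.
; The construction script optionally locks Y to zero, then sets spawn direction and preview arrow from Reverse.
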(event Custom|ClearHelp
  (bind _bpplatformercomponent (Variables|Default|GetBPPlatformerComponent))
  ;[0 1 0] Set last Check Point Position in Player, Play Sound, Display "Check Point" text and cut ropes
  (Utilities|IsValid _bpplatformercomponent
    (:Is%20Valid
      (Variables|/Game/PlatformTools/GameDefinitions/Components/BP_Platformer_Main.BP_Platformer_Main_C|SetHelperText _bpplatformercomponent ""))))

(event EventBeginPlay
  (bind _returnvalue (Game|GetPlayerCharacter 0))
  (bind _returnvalue_2 (Actor|GetComponentbyClass _returnvalue "/Game/PlatformTools/GameDefinitions/Components/BP_Platformer_Main.BP_Platformer_Main_C"))
  ;[1 1 0] Connect to Platformer_Main Component in Player
  (Utilities|FlowControl|Delay 0.2)
  (Utilities|IsValid _returnvalue_2
    (:Is%20Valid
      (Variables|Default|SetBPPlatformerComponent _returnvalue_2))))

(event Collision|EventActorBeginOverlap
  (params (OtherActor :type Actor%20Object%20Reference))
  (bind _bpplatformercomponent (Variables|Default|GetBPPlatformerComponent))
  ;[0 1 0] Set last Check Point Position in Player, Play Sound, Display "Check Point" text and cut ropes
  (if (== OtherActor (Game|GetPlayerCharacter 0))
    (Utilities|IsValid OtherActor
      (:Is%20Valid
        (Utilities|FlowControl|DoOnce false
          (:Completed
            (Audio|PlaySound2D (Variables|Default|GetSoundWave) 1.0 1.0 0.0 0 0)
            (Variables|/Script/CableComponent.CableComponent|SetbAttachEnd (Variables|Default|GetRopeLeft) false)
            (Variables|/Script/CableComponent.CableComponent|SetbAttachEnd (Variables|Default|GetRopeRIght) false)
            (Rendering|Material|SetMaterial (Variables|Default|GetSphereLeft) 0 (Variables|Materials|GetCPActivatedPattern))
            (Variables|/Game/PlatformTools/GameDefinitions/Components/BP_Platformer_Main.BP_Platformer_Main_C|SetHelperText _bpplatformercomponent "Check Point")
            (Variables|/Game/PlatformTools/GameDefinitions/Components/BP_Platformer_Main.BP_Platformer_Main_C|SetCheckPoint _bpplatformercomponent (Math|Transform|MakeTransform (+ (Transformation|GetWorldLocation (Variables|Default|GetSubScene)) (Variables|Default|GetPlayerHeightOffset)) (Variables|Default|GetCheckPointRotation) "1,1,1"))
            (Variables|/Game/PlatformTools/GameDefinitions/Components/BP_Platformer_Main.BP_Platformer_Main_C|SetZoomedIn _bpplatformercomponent (Variables|Default|GetZoomedIn))
            (Utilities|Time|SetTimerbyEvent (delegate Custom|ClearHelp) 2.0)))))))

(fn ConstructionScript
  (bind _basescene (Variables|Default|GetBaseScene))
  (bind _returnvalue (Transformation|GetWorldLocation _basescene))
  ;[0 1 0] Set the Material for the Spheres
  (Rendering|Material|SetMaterial (Variables|Default|GetSphereLeft) 0 (Variables|Materials|GetBasePattern))
  ;[1 0 0] Lock the Y axis to Zero
  (if (Variables|Default|GetLockY)
    (Transformation|SetWorldLocation (Variables|Default|GetBaseScene) (Math|Vector|MakeVector (.x _returnvalue) 0.0 (.z _returnvalue)) false false)
    ;[0 1 0] Set Arrow to Show Player Spawn Direction
    (if (Variables|Default|GetReverse)
      (Transformation|SetWorldRotation (Variables|Default|GetArrow) "0,180.000000, 0" false false)
      (Variables|Default|SetCheckPointRotation "0,90.000000, 0")
      (else
        (Transformation|SetWorldRotation (Variables|Default|GetArrow) "0, 0, 0" false false)
        (Variables|Default|SetCheckPointRotation "0.000000,-90.000000,0.000000")))))