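; Level finish line with a podium that ends a platformer level.
; Crossing it flags completion in the game instance, releases the ropes, recolors the spheres, saves a checkpoint through the player's platformer component and briefly shows "Finished!".
; Reaching the podium disables movement, swaps the game widget for the level-goal screen and blends to a spawned camera on the player.
; Trigger volumes toggle wall collision to confine the player to the finish area.
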(event OnComponentBeginOverlap(Box1)
  (params (OverlappedComponent :type Primitive%20Component%20Object%20Reference) (OtherActor :type Actor%20Object%20Reference) (OtherComp :type Primitive%20Component%20Object%20Reference) (OtherBodyIndex :type Integer) (bFromSweep :type Boolean) (SweepResult :type Hit%20Result%20Structure%20%28by%20ref%29))
  (bind _returnvalue (Viewport|GetViewportSize))
  ;[0 1 0] Check Player has Stood on Podium
  (if (== OtherActor (Game|GetPlayerCharacter 0))
    (Utilities|IsValid OtherActor
      (:Is%20Valid
        ;[1 0 0] Remove Game Widget
        (bind _foundwidgets (Widget|GetAllWidgetsOfClass "/Game/PlatformTools/UserInterfaces/Widget_Game.Widget_Game_C" true))
        (Widget|RemovefromParent (Utilities|Array|Get(acopy) _foundwidgets))
        ;[0 1 0] Display Level Goal Widget and commence Camera Zoom in on the Player
        (Variables|/Game/PlatformTools/GameDefinitions/Components/BP_Platformer_Main.BP_Platformer_Main_C|SetAllowMovement (Variables|Default|GetBPPlatformerComponent) false)
        (bind _returnvalue_2 (UserInterface|CreateWidget "/Game/PlatformTools/UserInterfaces/Widget_LevelGoal.Widget_LevelGoal_C" (Game|GetPlayerController 0)))
        (bind _output_get (Variables|Default|SetUILevelGoal _returnvalue_2))
        (UserInterface|Viewport|AddtoViewport _output_get 2)
        (Rendering|Material|SetMaterial (Variables|Default|GetPodiumBase) 0 "/Game/PlatformTools/LevelObjects/HelperObjects/CheckPoints/Materials/MI_Finish_Scroller.MI_Finish_Scroller")
        (bind _returnvalue_3 (Game|SpawnActorfromClass "/Script/Engine.CameraActor" (Math|Transform|MakeTransform (+ (Transformation|GetWorldLocation (Variables|/Script/Engine.Character|GetCapsuleComponent (Game|GetPlayerCharacter 0))) "275.000000,400.000000,0.000000") "0.000000,-90.000000, 0" "1,1,1") "Undefined" 0 0))
        (Class|CameraComponent|SetProjectionMode (Variables|/Script/Engine.CameraActor|GetCameraComponent _returnvalue_3) "Perspective")
        (Camera|SetFieldOfView (Variables|/Script/Engine.CameraActor|GetCameraComponent _returnvalue_3) 9e+01)
        (Variables|/Script/Engine.CameraComponent|SetbLockToHmd (Variables|/Script/Engine.CameraActor|GetCameraComponent _returnvalue_3) true)
        (Variables|/Script/Engine.CameraComponent|SetbConstrainAspectRatio (Variables|/Script/Engine.CameraActor|GetCameraComponent _returnvalue_3) true)
        (Class|CameraComponent|SetAspectRatio (Variables|/Script/Engine.CameraActor|GetCameraComponent _returnvalue_3) (/ (.x _returnvalue) (.y _returnvalue)))
        (Game|Player|SetViewTargetwithBlend (Game|GetPlayerController 0) _returnvalue_3 2.0 "VTBlend_Cubic" 1.0 false)))))

(event OnComponentEndOverlap(OneWayWall_Enter)
  (params (OverlappedComponent :type Primitive%20Component%20Object%20Reference) (OtherActor :type Actor%20Object%20Reference) (OtherComp :type Primitive%20Component%20Object%20Reference) (OtherBodyIndex :type Integer))
  (bind _returnvalue (Game|GetPlayerCharacter 0))
  ;[0 1 0] Ensure that once player crosses the Check Point, he can only move between the Check Point and the Podium
  (if (== OtherActor _returnvalue)
    (Utilities|IsValid OtherActor
      (:Is%20Valid
        (if (> (.y (Math|Vector|GetForwardVector (Variables|/Script/Engine.Character|GetMesh _returnvalue))) 0.0)
          (Collision|SetCollisionProfileName (Variables|Default|GetOneWayWall_Enter) "OverlapAll" :!class /Script/Engine.PrimitiveComponent)
          (else
            (Collision|SetCollisionProfileName (Variables|Default|GetOneWayWall_Enter) "BlockAll" :!class /Script/Engine.PrimitiveComponent)))))))

(event OnComponentBeginOverlap(OneWayWall_Exit)
  (params (OverlappedComponent :type Primitive%20Component%20Object%20Reference) (OtherActor :type Actor%20Object%20Reference) (OtherComp :type Primitive%20Component%20Object%20Reference) (OtherBodyIndex :type Integer) (bFromSweep :type Boolean) (SweepResult :type Hit%20Result%20Structure%20%28by%20ref%29))
  ;[0 1 0] Esnure the Player Cannot Move Past the Podium
  (if (== OtherActor (Game|GetPlayerCharacter 0))
    (Utilities|IsValid OtherActor
      (:Is%20Valid
        (Collision|SetCollisionProfileName (Variables|Default|GetOneWayWall_Enter) "BlockAll" :!class /Script/Engine.PrimitiveComponent)))))

(event OnComponentBeginOverlap(Box)
  (params (OverlappedComponent :type Primitive%20Component%20Object%20Reference) (OtherActor :type Actor%20Object%20Reference) (OtherComp :type Primitive%20Component%20Object%20Reference) (OtherBodyIndex :type Integer) (bFromSweep :type Boolean) (SweepResult :type Hit%20Result%20Structure%20%28by%20ref%29))
  (bind _subscene (Variables|Default|GetSubScene))
  (bind _bpplatformercomponent (Variables|Default|GetBPPlatformerComponent))
  ;[0 1 0] Confirm the Player is Crossing the Line
  (if (== OtherActor (Game|GetPlayerCharacter 0))
    (Utilities|IsValid OtherActor
      (:Is%20Valid
        (Utilities|FlowControl|DoOnce false
          (:Completed
            ;[1 0 0] Stop Timers
            (bind _asgame_instance_platformer (Utilities|Casting|CastToGameInstance_Platformer (Game|GetGameInstance)))
            (Variables|/Game/PlatformTools/GameDefinitions/GameInstance_Platformer.GameInstance_Platformer_C|SetLevelComplete _asgame_instance_platformer true)
            ;[0 1 0] Detach Ropes, Set Sphere Materials, Helper Text and Play Sounds
            (Variables|/Script/CableComponent.CableComponent|SetbAttachEnd (Variables|Default|GetRopeLeft) false)
            (Variables|/Script/CableComponent.CableComponent|SetbAttachEnd (Variables|Default|GetRopeRIght) false)
            (Rendering|Material|SetMaterial (Variables|Default|GetSphereLeft) 0 (Variables|Materials|GetCPActivatedPattern))
            (Variables|/Game/PlatformTools/GameDefinitions/Components/BP_Platformer_Main.BP_Platformer_Main_C|SetHelperText _bpplatformercomponent "Finished!")
            (Variables|/Game/PlatformTools/GameDefinitions/Components/BP_Platformer_Main.BP_Platformer_Main_C|SetCheckPoint _bpplatformercomponent (Math|Transform|MakeTransform (+ (Transformation|GetWorldLocation _subscene) (Variables|Default|GetPlayerHeightOffset)) (Math|Rotator|CombineRotators (Transformation|GetWorldRotation _subscene) (Variables|Default|GetPlayerDefaultRotation)) "1,1,1"))
            (Audio|PlaySound2D (Variables|Default|GetSoundWave) 1.0 1.0 0.0 0 0)
            (Utilities|Time|SetTimerbyEvent (delegate Custom|ClearHelp) 2.0)))))))

(event Custom|ClearHelp
  (bind _bpplatformercomponent (Variables|Default|GetBPPlatformerComponent))
  ;[0 1 0] Detach Ropes, Set Sphere Materials, Helper Text and Play Sounds
  (Utilities|IsValid _bpplatformercomponent
    (:Is%20Valid
      (Variables|/Game/PlatformTools/GameDefinitions/Components/BP_Platformer_Main.BP_Platformer_Main_C|SetHelperText _bpplatformercomponent ""))))

(event EventBeginPlay
  (bind _returnvalue (Game|GetPlayerCharacter 0))
  (bind _returnvalue_2 (Actor|GetComponentbyClass _returnvalue "/Game/PlatformTools/GameDefinitions/Components/BP_Platformer_Main.BP_Platformer_Main_C"))
  ;[1 1 0] Connect to Platformer_Main Component in Player
  (Utilities|FlowControl|Delay 0.2)
  (Utilities|IsValid _returnvalue_2
    (:Is%20Valid
      (Variables|Default|SetBPPlatformerComponent _returnvalue_2))))

(fn ConstructionScript
  (bind _basescene (Variables|Default|GetBaseScene))
  (bind _returnvalue (Transformation|GetWorldLocation _basescene))
  ;[0 1 0] Set the Material for the Spheres
  (Rendering|Material|SetMaterial (Variables|Default|GetSphereLeft) 0 (Variables|Materials|GetBasePattern))
  ;[1 0 0] Lock the Y axis to Zero
  (if (Variables|Default|GetLockY)
    (Transformation|SetWorldLocation (Variables|Default|GetBaseScene) (Math|Vector|MakeVector (.x _returnvalue) 0.0 (.z _returnvalue)) false false)))