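; BP_LoadStreamLevel is a placeable trigger that streams in a named level when the player character enters its box, to improve mobile performance.
; The first player overlap passes a DoOnce and starts a non-blocking load that makes the level visible once loaded.
; The construction script shows the level name on a text render.
; With LockY enabled, the scene root snaps to world Y zero at construction and after triggering.
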(event OnComponentBeginOverlap(Box)
  (params (OverlappedComponent :type Primitive%20Component%20Object%20Reference) (OtherActor :type Actor%20Object%20Reference) (OtherComp :type Primitive%20Component%20Object%20Reference) (OtherBodyIndex :type Integer) (bFromSweep :type Boolean) (SweepResult :type Hit%20Result%20Structure%20%28by%20ref%29))
  (bind _scene (Variables|Default|GetScene))
  (bind _returnvalue (Transformation|GetWorldLocation _scene))
  ;[0 1 0] Load a Steaming Level with the Specified Name (Improves Mobile Performance)
  (if (== OtherActor (Game|GetPlayerCharacter 0))
    (Utilities|FlowControl|DoOnce false
      (:Completed
        (Game|LoadStreamLevel(byName) (Utilities|String|StringToName (Variables|Default|GetLevelName)) true)
        (if (Variables|Default|GetLockY)
          ;[1 0 0] Lock Y at 0
          (Transformation|SetWorldLocation (Variables|Default|GetScene) (Math|Vector|MakeVector (.x _returnvalue) 0.0 (.z _returnvalue)) false false))))))

(fn ConstructionScript
  (bind _scene (Variables|Default|GetScene))
  (bind _returnvalue (Transformation|GetWorldLocation _scene))
  (Utilities|FlowControl|Sequence
    (:then_0
      (if (Variables|Default|GetLockY)
        ;[1 0 0] Lock Y at 0
        (Transformation|SetWorldLocation (Variables|Default|GetScene) (Math|Vector|MakeVector (.x _returnvalue) 0.0 (.z _returnvalue)) false false)))
    (:then_1
      ;[0 1 0] Show Level Name to Stream In as Text Render
      (Rendering|Components|TextRender|SetText (Variables|Default|GetTextRender) (Utilities|Text|ToText(String) (Variables|Default|GetLevelName))))))