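; BP_Information is an info sign for a platformer level that shows help text when the player enters its box trigger.
; It caches the player's BP_Platformer_Main component shortly after BeginPlay and notifies it on overlap begin and end, delaying the end call by a configurable display time.
; The sign also toggles DisplayAdvert on the Widget_Game HUD.
; An optional construction-script lock pins the sign to Y zero.
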(event OnComponentBeginOverlap(Box)
  (params (OverlappedComponent :type Primitive%20Component%20Object%20Reference) (OtherActor :type Actor%20Object%20Reference) (OtherComp :type Primitive%20Component%20Object%20Reference) (OtherBodyIndex :type Integer) (bFromSweep :type Boolean) (SweepResult :type Hit%20Result%20Structure%20%28by%20ref%29))
  ;[0 1 0] Handles Overlap of the Player
  (if (== OtherActor (Game|GetPlayerCharacter 0))
    (Utilities|IsValid OtherActor
      (:Is%20Valid
        (Default|CallInfoSignEventBeginOverlap (Variables|Default|GetBPPlatformerComponent) (Variables|Default|GetHelpText))
        (bind _foundwidgets (Widget|GetAllWidgetsOfClass "/Game/PlatformTools/UserInterfaces/Widget_Game.Widget_Game_C" false))
        (Variables|/Game/PlatformTools/UserInterfaces/Widget_Game.Widget_Game_C|SetDisplayAdvert (Utilities|Array|Get(acopy) _foundwidgets) (Variables|Default|GetDisplayAdvert))))))

(event OnComponentEndOverlap(Box)
  (params (OverlappedComponent :type Primitive%20Component%20Object%20Reference) (OtherActor :type Actor%20Object%20Reference) (OtherComp :type Primitive%20Component%20Object%20Reference) (OtherBodyIndex :type Integer))
  ;[1 0 0] Once the Player Has Moved Past the Sign, Display Text for %DisplayTime% Seconds.
  (if (== OtherActor (Game|GetPlayerCharacter 0))
    (Utilities|IsValid OtherActor
      (:Is%20Valid
        (Utilities|FlowControl|Delay (Variables|Default|GetDisplayTime))
        (Default|CallInfoSignEventEndOverlap (Variables|Default|GetBPPlatformerComponent))
        (bind _foundwidgets (Widget|GetAllWidgetsOfClass "/Game/PlatformTools/UserInterfaces/Widget_Game.Widget_Game_C" false))
        (Variables|/Game/PlatformTools/UserInterfaces/Widget_Game.Widget_Game_C|SetDisplayAdvert (Utilities|Array|Get(acopy) _foundwidgets) false)))))

(event EventBeginPlay
  (bind _returnvalue (Game|GetPlayerCharacter 0))
  (bind _returnvalue_2 (Actor|GetComponentbyClass _returnvalue "/Game/PlatformTools/GameDefinitions/Components/BP_Platformer_Main.BP_Platformer_Main_C"))
  ;[1 1 0] Connect to Platformer_Main Component in Player
  (Utilities|FlowControl|Delay 0.2)
  (Utilities|IsValid _returnvalue_2
    (:Is%20Valid
      (Variables|Default|SetBPPlatformerComponent _returnvalue_2))))

(fn ConstructionScript
  (bind _scene (Variables|Default|GetScene))
  (bind _returnvalue (Transformation|GetWorldLocation _scene))
  (if (Variables|Default|GetLockY)
    ;[1 0 0] Lock Y at 0
    (Transformation|SetWorldLocation (Variables|Default|GetScene) (Math|Vector|MakeVector (.x _returnvalue) 0.0 (.z _returnvalue)) false false)))