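; BP_ZoomIn is a level helper trigger that moves the player's camera between zoomed-out and zoomed-in positions.
; When the player overlaps the box, it takes endpoints from the platformer GameInstance, optionally overriding the zoom-in position.
; Mesh facing along Y and a Reverse flag decide direction, then a ZoomTime-scaled timeline lerps the camera's relative location unless already there.
; Construction labels it with its display name and optionally locks Y to zero.
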(event OnComponentBeginOverlap(Box)
  (params (OverlappedComponent :type Primitive%20Component%20Object%20Reference) (OtherActor :type Actor%20Object%20Reference) (OtherComp :type Primitive%20Component%20Object%20Reference) (OtherBodyIndex :type Integer) (bFromSweep :type Boolean) (SweepResult :type Hit%20Result%20Structure%20%28by%20ref%29))
  (bind _returnvalue (Game|GetPlayerCharacter 0))
  (bind _mesh (Variables|/Script/Engine.Character|GetMesh _returnvalue))
  (bind _returnvalue_2 (Math|Vector|GetForwardVector _mesh))
  (bind _returnvalue_3 (Math|Float|Sign(Float) (.y _returnvalue_2)))
  (bind _returnvalue_4 (< _returnvalue_3 0.0))
  ;[0 1 0] Handle Player Overlap of ZoomIn
  (if (== OtherActor (Game|GetPlayerCharacter 0))
    (Variables|Default|SetCurrentZoom (Variables|/Script/Engine.SceneComponent|GetRelativeLocation (Utilities|Array|Get(acopy) (Actor|GetComponentsByClass (Game|GetPlayerCharacter 0) "/Script/Engine.CameraComponent"))))
    (if (Variables|Default|GetOverrideZoom)
      (Variables|Default|SetEndZoom (Variables|Default|GetZoomInOverride))
      (else
        (bind _asgame_instance_platformer (Utilities|Casting|CastToGameInstance_Platformer (Game|GetGameInstance)))
        (Variables|Default|SetEndZoom (.location (Variables|/Game/PlatformTools/GameDefinitions/GameInstance_Platformer.GameInstance_Platformer_C|GetDefaultPlayerCameraLoc _asgame_instance_platformer)))))
    (Variables|Default|SetStartZoom (.location (Variables|/Game/PlatformTools/GameDefinitions/GameInstance_Platformer.GameInstance_Platformer_C|GetZoomOutPlayerCameraLoc _asgame_instance_platformer)))
    (if (Variables|Default|GetReverse)
      (if _returnvalue_4
        (Variables|Default|SetTempZoom (Variables|Default|GetStartZoom) :!label _label)
        (Variables|Default|SetStartZoom (Variables|Default|GetEndZoom))
        (Variables|Default|SetEndZoom (Variables|Default|GetTempZoom)))
      (elif _returnvalue_4
        _
        (else
          (goto _label))))
    (Components|Timeline|SetPlayRate (Variables|Default|GetCameraZoom_Timeline) (/ 1.0 (Variables|Default|GetZoomTime)))
    (if (not (Math|Vector|Equal(Vector) (Variables|Default|GetCurrentZoom) (Variables|Default|GetEndZoom) 0.0001))
      (bind _fade (Timeline|CameraZoom_Timeline PlayFromStart)
        (:Update
          (Transformation|SetRelativeLocation (Utilities|Array|Get(acopy) (Actor|GetComponentsByClass (Game|GetPlayerCharacter 0) "/Script/Engine.CameraComponent")) (Math|Vector|Lerp(Vector) (Variables|Default|GetStartZoom) (Variables|Default|GetEndZoom) _fade) false false))))))

(fn ConstructionScript
  (bind _scene (Variables|Default|GetScene))
  (bind _returnvalue (Transformation|GetWorldLocation _scene))
  ;[0 1 0] Set Render Text
  (Rendering|Components|TextRender|SetText (Variables|Default|GetTextRender) (Utilities|Text|ToText(String) (Utilities|GetDisplayName self)))
  (if (Variables|Default|GetLockY)
    ;[1 0 0] Lock Y at 0
    (Transformation|SetWorldLocation (Variables|Default|GetScene) (Math|Vector|MakeVector (.x _returnvalue) 0.0 (.z _returnvalue)) false false)))