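; BP_CharacterSwitcher previews the selected player class via a child actor in what appears to be a menu, with custom colors.
; On the game instance's class-update event, or shortly after BeginPlay, it swaps the actor class and transform, targets the menu camera and zeroes player gravity.
; Color updates skip the swap.
; For custom-color classes, matching skeletal mesh slots get dynamic materials with RGB tints, each brightness overridden through HSV.
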(event Custom|ChangeMesh
  (bind _returnvalue (Game|GetPlayerCharacter 0))
  ;[0 1 0] Setup Character Switcher, Dispatchers and Color Changes
  (bind _asgame_instance_platformer (Utilities|Casting|CastToGameInstance_Platformer (Game|GetGameInstance)))
  (Utilities|IsValid _asgame_instance_platformer
    (:Is%20Valid
      (if (Variables|Default|GetSkipActorChange)
        _
        (else
          (Transformation|SetRelativeTransform (Variables|Default|GetChildActor) (.MenuTransform (Utilities|Struct|BreakStruct_Characters (Utilities|Array|Get(acopy) (Variables|/Game/PlatformTools/GameDefinitions/GameInstance_Platformer.GameInstance_Platformer_C|GetCharacter _asgame_instance_platformer) (Math|Conversions|ToInteger(Byte) (Variables|/Game/PlatformTools/GameDefinitions/GameInstance_Platformer.GameInstance_Platformer_C|GetPlayerClass _asgame_instance_platformer))))) false false)
          (ChildActorComponent|SetChildActorClass (Variables|Default|GetChildActor) (.PlayerBP (Utilities|Struct|BreakStruct_Characters (Utilities|Array|Get(acopy) (Variables|/Game/PlatformTools/GameDefinitions/GameInstance_Platformer.GameInstance_Platformer_C|GetCharacter _asgame_instance_platformer) (Math|Conversions|ToInteger(Byte) (Variables|/Game/PlatformTools/GameDefinitions/GameInstance_Platformer.GameInstance_Platformer_C|GetPlayerClass _asgame_instance_platformer))))))
          (Game|Player|SetViewTargetwithBlend (Game|GetPlayerController 0) (Variables|/Game/PlatformTools/GameDefinitions/GameInstance_Platformer.GameInstance_Platformer_C|GetMenuCamBPLink _asgame_instance_platformer) 0.0 "VTBlend_Linear" 0.0 false)
          (Utilities|IsValid _returnvalue
            (:Is%20Valid
              (Variables|/Script/Engine.CharacterMovementComponent|SetGravityScale (Variables|/Script/Engine.Character|GetCharacterMovement _returnvalue) 0.0)))))
      (if (.UseCustomColors (Utilities|Struct|BreakStruct_Characters (Utilities|Array|Get(acopy) (Variables|/Game/PlatformTools/GameDefinitions/GameInstance_Platformer.GameInstance_Platformer_C|GetCharacter _asgame_instance_platformer) (Math|Conversions|ToInteger(Byte) (Variables|/Game/PlatformTools/GameDefinitions/GameInstance_Platformer.GameInstance_Platformer_C|GetPlayerClass _asgame_instance_platformer)))))
        (Variables|Default|SetSkipActorChange false)
        (bind _integer (CallFunction|GetMaterialSlot))
        (bind _asskeletal_mesh_component (Utilities|Casting|CastToSkeletalMeshComponent (Utilities|Array|Get(acopy) (Components|GetChildrenComponents (Variables|Default|GetChildActor) true) _integer))
          (:then
            (bind _output_get (Variables|Default|SetChildMesh _asskeletal_mesh_component))
            (for (_ _array_index) (Rendering|Material|GetMaterials _output_get)
              (for _array_element (Variables|/Game/PlatformTools/GameDefinitions/GameInstance_Platformer.GameInstance_Platformer_C|GetCharacter_Materials _asgame_instance_platformer)
                (if (== (.playerclass _array_element) (Math|Conversions|ToInteger(Byte) (Variables|/Game/PlatformTools/GameDefinitions/GameInstance_Platformer.GameInstance_Platformer_C|GetPlayerClass _asgame_instance_platformer)))
                  (if (== _array_index (.dmat_materialslotnumber _array_element))
                    (bind _returnvalue_2 (Rendering|Material|CreateDynamicMaterialInstance (.materialname _array_element) "None" :!class /Script/Engine.KismetMaterialLibrary))
                    (Utilities|IsValid _returnvalue_2
                      (:Is%20Valid
                        (Rendering|Material|SetMaterial (Variables|Default|GetChildMesh) _array_index _returnvalue_2)
                        (Rendering|Material|SetVectorParameterValue _returnvalue_2 "BaseColorR" (Class|KismetMathLibrary|HSVtoRGB (.H (Math|Color|RGBtoHSV(LinearColor) (.r_color _array_element))) (.S (Math|Color|RGBtoHSV(LinearColor) (.r_color _array_element))) (.r_value _array_element) 1.0) :!class /Script/Engine.MaterialInstanceDynamic)
                        (Rendering|Material|SetVectorParameterValue _returnvalue_2 "BaseColorG" (Class|KismetMathLibrary|HSVtoRGB (.H (Math|Color|RGBtoHSV(LinearColor) (.g_color _array_element))) (.S (Math|Color|RGBtoHSV(LinearColor) (.g_color _array_element))) (.g_value _array_element) 1.0) :!class /Script/Engine.MaterialInstanceDynamic)
                        (Rendering|Material|SetVectorParameterValue _returnvalue_2 "BaseColorB" (Class|KismetMathLibrary|HSVtoRGB (.H (Math|Color|RGBtoHSV(LinearColor) (.b_color _array_element))) (.S (Math|Color|RGBtoHSV(LinearColor) (.b_color _array_element))) (.b_value _array_element) 1.0) :!class /Script/Engine.MaterialInstanceDynamic)
                        (Variables|Default|SetMatMatched true))))))
              (if (Variables|Default|GetMatMatched)
                (Variables|Default|SetMatMatched false))))
          (:CastFailed
            (Development|PrintString "Cast Failed")))))))

(event Custom|UpdateColors
  ;[0 1 0] Setup Character Switcher, Dispatchers and Color Changes
  (Variables|Default|SetSkipActorChange true)
  (CallFunction|ChangeMesh))

(event EventBeginPlay
  ;[0 1 0] Setup Character Switcher, Dispatchers and Color Changes
  (EventDispatchers|BindEventtoUpdateClassEvent (delegate Custom|ChangeMesh))
  (EventDispatchers|BindEventtoUpdateColorsEvent (delegate Custom|UpdateColors))
  (Utilities|FlowControl|Delay 0.2)
  (CallFunction|ChangeMesh))

(fn ConstructionScript)

(fn GetMaterialSlot
  (for (_array_element _array_index) (Components|GetChildrenComponents (Variables|Default|GetChildActor) true)
    (if (== (Utilities|GetClass _array_element) "/Script/Engine.SkeletalMeshComponent")
      (return _array_index))))